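; Stage actor that renders selection thumbnails at BeginPlay for every BP_EditableObject's base and switching options, unless an override thumbnail exists.
; Each option gets a mesh component (its own or a preview mesh) with materials applied, framed by bounds and FOV.
; A new scene capture per option hides the other spawned meshes and writes to a render target stored on the object.
; Captures render every frame until deactivated after RenderTime.
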(event EventBeginPlay
  (Rendering|SetVisibility (Variables|Default|GetRenderMesh) false false)
  (Utilities|FlowControl|Sequence
    (:then_0
      ;[1 1 1] Render Meshes
      (bind _outactors (Actor|GetAllActorsOfClass "/Game/HALArchvizToolkit/Blueprints/BP_EditableObject.BP_EditableObject_C"))
      (for _array_element _outactors
        (CallFunction|RenderThumbnail _array_element)))
    (:then_2
      ;[1 1 1] Turn off captures
      (Utilities|FlowControl|Delay (Variables|Thumbnails|GetRenderTime))
      (Components|Activation|SetActive (Variables|Default|Get2DCaptures) false false))))

(fn ConstructionScript
  (Variables|/Script/Engine.SceneCaptureComponent2D|SetFOVAngle (Variables|Default|GetSceneCaptureComponent2D) (Variables|Thumbnails|GetFOV))
  (Transformation|AddLocalOffset (Variables|Default|GetCamera) "0.100000,0.000000, 0" false))

(fn RenderThumbnail
  (params (EditableObject :type BP%20Editable%20Object%20Object%20Reference%20%28by%20ref%29))
  (bind _thumbnailsize (Variables|Thumbnails|GetThumbnailSize))
  (bind _output_get (LocalVariables|SetCurrentEditableObject EditableObject))
  ;[1 1 1] Build Arrays and cache local vars
  (Utilities|IsValid (Variables|/Game/HALArchvizToolkit/Blueprints/BP_EditableObject.BP_EditableObject_C|GetBaseMesh _output_get)
    (:Is%20Valid
      (LocalVariables|SetUseMesh (Variables|/Game/HALArchvizToolkit/Blueprints/BP_EditableObject.BP_EditableObject_C|GetUseMeshForThumbnails _output_get))
      (Utilities|Array|Add (LocalVariables|GetCurrentChoicesArray) (Utilities|Struct|MakeObjectChoices (Variables|/Game/HALArchvizToolkit/Blueprints/BP_EditableObject.BP_EditableObject_C|GetBaseMesh _output_get) (Variables|/Game/HALArchvizToolkit/Blueprints/BP_EditableObject.BP_EditableObject_C|GetBaseMaterials _output_get) (Variables|/Game/HALArchvizToolkit/Blueprints/BP_EditableObject.BP_EditableObject_C|GetBaseThumbnail _output_get)))
      (Utilities|Array|AppendArray (LocalVariables|GetCurrentChoicesArray) (Variables|/Game/HALArchvizToolkit/Blueprints/BP_EditableObject.BP_EditableObject_C|GetSwitchingOptions _output_get))
      (Utilities|Array|Clear (Variables|/Game/HALArchvizToolkit/Blueprints/BP_EditableObject.BP_EditableObject_C|GetSelectionThumbnails _output_get))
      ;[1 1 1] Loop through each switching option
      (for (_array_element _array_index) (LocalVariables|GetCurrentChoicesArray)
        (LocalVariables|SetIndex _array_index)
        (Utilities|IsValid (.thumbnailoverride _array_element) ; If a Thumbnail is already defined, use that\nElse, render a thumbnail
          (:Is%20Valid
            ;[1 1 1] If a thumbnail is defined, use that and skip everything else
            (Utilities|Array|Add (Variables|/Game/HALArchvizToolkit/Blueprints/BP_EditableObject.BP_EditableObject_C|GetSelectionThumbnails (LocalVariables|GetCurrentEditableObject)) (.thumbnailoverride _array_element)))
          (:Is%20Not%20Valid
            ;[1 1 1] Local variables
            (LocalVariables|SetCurrentMaterials (.materialoverrides _array_element))
            (LocalVariables|SetCurrentMesh (select (Utilities|IsValid (.meshoverride _array_element)) (.meshoverride _array_element) (Variables|/Game/HALArchvizToolkit/Blueprints/BP_EditableObject.BP_EditableObject_C|GetBaseMesh (LocalVariables|GetCurrentEditableObject))))
            (Utilities|FlowControl|Sequence
              (:then_1
                ;[1 1 1] Create Mesh component and hide from any existing scene captures
                (if (LocalVariables|GetUseMesh)
                  ;;[0.5482 1 0.7914] Base or Override mesh
                  (bind _returnvalue (AddComponent|AddStaticMeshComponent false))
                  (bind _output_get_2 (LocalVariables|SetCurrentComponent _returnvalue))
                  (Components|StaticMesh|SetStaticMesh _output_get_2 (LocalVariables|GetCurrentMesh))
                  (Utilities|FlowControl|Sequence
                    (:then_0
                      ;;[1 1 1] Rotate direction of mesh
                      (Utilities|IsValid (LocalVariables|GetCurrentComponent)
                        (:Is%20Valid
                          (switch Utilities|FlowControl|Switch|SwitchonE_AxisDirections (Variables|/Game/HALArchvizToolkit/Blueprints/BP_EditableObject.BP_EditableObject_C|GetRenderAxis (LocalVariables|GetCurrentEditableObject))
                            (:NewEnumerator0
                              (Transformation|SetRelativeRotation (LocalVariables|GetCurrentComponent) "0,0.000000, 0" false))
                            (:NewEnumerator2
                              (Transformation|SetRelativeRotation (LocalVariables|GetCurrentComponent) "0,180.000000, 0" false))
                            (:NewEnumerator1
                              (Transformation|SetRelativeRotation (LocalVariables|GetCurrentComponent) "0,-90.000000, 0" false))
                            (:NewEnumerator3
                              (Transformation|SetRelativeRotation (LocalVariables|GetCurrentComponent) "0,90.000000, 0" false))))))
                    (:then_1
                      ;;[0.4967 1 0.6563] Set materials
                      (for (_array_element_2 _array_index_2) (LocalVariables|GetCurrentMaterials) :!label _label ; Material overrides
                        (if (Utilities|IsValid _array_element_2)
                          (Rendering|Material|SetMaterial (LocalVariables|GetCurrentComponent) _array_index_2 _array_element_2)))
                      ;;[0.5116 1 0.654] Set Location to center of stage
                      (Transformation|SetRelativeLocation (LocalVariables|GetCurrentComponent) (Math|Vector|MakeVector 0.0 0.0 (* (.z (.Min (Components|StaticMesh|GetLocalBounds (LocalVariables|GetCurrentComponent)))) -1.0)) false :!label _label_2)
                      ;;[1 1 1] Hide from existing scene captures
                      (for _array_element_3 (Variables|Default|Get2DCaptures)
                        (Class|SceneCaptureComponent|HideComponent _array_element_3 (LocalVariables|GetCurrentComponent)))))
                  (else
                    ;;[0.5692 1 0.8435] PreviewMesh
                    (bind _returnvalue_2 (AddComponent|AddStaticMeshComponent false))
                    (bind _output_get_3 (LocalVariables|SetCurrentComponent _returnvalue_2))
                    (Components|StaticMesh|SetStaticMesh _output_get_3 (Variables|Thumbnails|GetPreviewMesh))
                    (if (> (Utilities|Array|Length (LocalVariables|GetCurrentMaterials)) 0)
                      (goto _label)
                      (else
                        (for (_array_element_4 _array_index_3) (Variables|/Game/HALArchvizToolkit/Blueprints/BP_EditableObject.BP_EditableObject_C|GetBaseMeshMaterials (LocalVariables|GetCurrentEditableObject)) ; Material overrides
                          (if (Utilities|IsValid _array_element_4)
                            (Rendering|Material|SetMaterial (LocalVariables|GetCurrentComponent) _array_index_3 _array_element_4)))
                        (goto _label_2))))))
              (:then_2
                ;[1 1 1] Position the camera based on the mesh
                (Utilities|IsValid (LocalVariables|GetCurrentComponent)
                  (:Is%20Valid
                    (Transformation|SetRelativeLocation (Variables|Default|GetCameraGimbal) (- (.Origin (Collision|GetComponentBounds (LocalVariables|GetCurrentComponent))) (Transformation|GetActorLocation)) false)
                    (Transformation|SetRelativeLocation (Variables|Default|GetCamera) (Math|Vector|MakeVector (* (/ (.SphereRadius (Collision|GetComponentBounds (LocalVariables|GetCurrentComponent))) (Math|Trig|Sin(Radians) (/ (Math|Trig|DegreesToRadians (Variables|Thumbnails|GetFOV)) 2.0))) -1.0) 0.0 0.0) false))))
              (:then_3
                ;[1 1 1] Render Mesh
                (bind _returnvalue_3 (AddComponent|AddSceneCaptureComponent2D true (Class|KismetMathLibrary|ConvertTransformtoRelative (Transformation|GetWorldTransform (Variables|Default|GetSceneCaptureComponent2D)))))
                (Utilities|IsValid _returnvalue_3
                  (:Is%20Valid
                    (for _array_element_5 (Variables|Default|GetStaticMeshComponents)
                      (Class|SceneCaptureComponent|HideComponent _returnvalue_3 _array_element_5))
                    (Utilities|Array|Add (Variables|Default|GetStaticMeshComponents) (LocalVariables|GetCurrentComponent))
                    (bind _returnvalue_4 (CanvasRenderTarget2D|CreateCanvasRenderTarget2D "/Game/HALArchvizToolkit/Blueprints/Resources/DynamicRender.DynamicRender_C" _thumbnailsize _thumbnailsize))
                    (bind _output_get_4 (Variables|/Script/Engine.SceneCaptureComponent2D|SetTextureTarget _returnvalue_3 _returnvalue_4))
                    (Utilities|Array|Add (Variables|Default|Get2DCaptures) _returnvalue_3)
                    (Variables|/Script/Engine.SceneCaptureComponent2D|SetCaptureSource _returnvalue_3 "SCS_FinalColorLDR")
                    (Variables|/Script/Engine.SceneCaptureComponent|SetbCaptureEveryFrame _returnvalue_3 true)
                    (Variables|/Script/Engine.SceneCaptureComponent2D|SetPostProcessSettings _returnvalue_3 (Variables|/Script/Engine.SceneCaptureComponent2D|GetPostProcessSettings (Variables|Default|GetSceneCaptureComponent2D)))
                    (Variables|/Script/Engine.SceneCaptureComponent2D|SetFOVAngle _returnvalue_3 (Variables|Thumbnails|GetFOV)))))
              (:then_4
                ;[0.6113 1 0.108] Set Texture on target
                (Utilities|Array|Add (Variables|/Game/HALArchvizToolkit/Blueprints/BP_EditableObject.BP_EditableObject_C|GetSelectionThumbnails (LocalVariables|GetCurrentEditableObject)) _output_get_4))
              (:then_5
                ;[1 1 1] PreviewCubes
                (if (Variables|Thumbnails|GetShowDebugCubes)
                  (bind _returnvalue_5 (AddComponent|AddStaticMeshComponent false))
                  (Components|StaticMesh|SetStaticMesh _returnvalue_5 "/Engine/BasicShapes/Cube.Cube")
                  (bind _returnvalue_6 (Rendering|Material|CreateDynamicMaterialInstance "/Game/HALArchvizToolkit/Blueprints/Resources/M_Thumbnail.M_Thumbnail" :!class /Script/Engine.KismetMaterialLibrary))
                  (Rendering|Material|SetTextureParameterValue _returnvalue_6 "TextureMap" _output_get_4)
                  (Rendering|Material|SetMaterial _returnvalue_5 0 _returnvalue_6)
                  (Transformation|AddLocalOffset _returnvalue_5 (Math|Vector|MakeVector 5e+02 5e+02 (* (LocalVariables|GetIndex) 1.1e+02)) false))))))))
    (:Is%20Not%20Valid
      (Development|PrintString "No Base Mesh Defined!" false false "(R=1.000000,G=0.053491,B=0.000000,A=1.000000)"))))

(fn FindMatchingChoice
  (params (InArray :type Array%20of%20Object%20Choices%20Structures) (InChoice :type Object%20Choices%20Structure))
  (bind (_meshoverride _materialoverrides) (Utilities|Struct|BreakObjectChoices InChoice))
  (bind (_array_element _array_index) (Utilities|Array|ForEachLoopwithBreak (Variables|Default|GetRenderedOptionsArray) :!label _label)
    (:LoopBody
      (if (== (.MeshOverride (Utilities|Struct|BreakObjectChoices _array_element)) _meshoverride)
        (bind (_array_element_2 _array_index_2) (Utilities|Array|ForEachLoopwithBreak (.MaterialOverrides (Utilities|Struct|BreakObjectChoices _array_element)) :!label _label_2)
          (:LoopBody
            (if (not (== _array_element_2 (Utilities|Array|Get(acopy) _materialoverrides _array_index_2)))
              (LocalVariables|SetModelMatchBreak true)
              (goto _label_2 Break)))
          (:Completed
            (if (not (LocalVariables|GetMaterialMatchBreak))
              (LocalVariables|SetReturnIndex _array_index)
              (return (LocalVariables|GetReturnIndex)))))
        (else
          (goto _label Break))))
    (:Completed
      (return (LocalVariables|GetReturnIndex)))))