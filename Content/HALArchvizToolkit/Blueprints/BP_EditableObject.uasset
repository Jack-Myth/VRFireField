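; Editable archviz actor that switches between a base mesh and configured mesh or material options.
; The construction script prebuilds a component per mesh override, reusing the base otherwise, plus optional bounds-sized box collision.
; SwitchModel activates the MeshIndex entry, applying materials, Pawn collision response and custom depth, and syncs the invisible ShadowMesh.
; BeginPlay fills selection thumbnails from overrides when no BP_ThumbnailRenderStage exists.
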(event `self.ReceiveBeginPlay`
  ;[1 1 1] Get Thumbnail Overrides if Render Stage Doesn't Exist
  (if (not (`self.RenderStageExists`))
    (`KismetArrayLibrary.Array_Add` (`self.SelectionThumbnails`) (`self.BaseThumbnail`))
    (for _array_element (`self.SwitchingOptions`)
      (`KismetArrayLibrary.Array_Add` (`self.SelectionThumbnails`) (`.ThumbnailOverride_40_C82AFAFB41A2EFE5B3641793ADD735CB` (break `/Game/HALArchvizToolkit/Blueprints/ObjectChoices` _array_element))))))

(event `self.ReceiveActorBeginOverlap`
  (params (OtherActor :type "Actor Object Reference")))

(event `self.ReceiveTick`
  (params (DeltaSeconds :type "Float (single-precision)")))

(event `/Game/HALArchvizToolkit/Blueprints/HUDInterface.SwitchModel`
  (bind _shadowmesh (`self.ShadowMesh`))
  (bind _meshcomponents (`self.MeshComponents`))
  (bind _meshindex (`self.MeshIndex`))
  (bind _item (`KismetArrayLibrary.Array_Get` _meshcomponents _meshindex))
  (bind _item_2 (`KismetArrayLibrary.Array_Get` (`self.MeshComponents`) (`self.MeshIndex`)))
  (bind _returnvalue (`MeshComponent.GetMaterials` (`KismetArrayLibrary.Array_Get` (`self.MeshComponents`) (`self.MeshIndex`))))
  (bind (_meshoverride _materialoverrides) (break `/Game/HALArchvizToolkit/Blueprints/ObjectChoices` (`KismetArrayLibrary.Array_Get` (`self.SwitchingOptions`) (- (`self.MeshIndex`) 1))))
  (`PrimitiveComponent.SetRenderCustomDepth` _meshcomponents false)
  (`SceneComponent.SetVisibility` _meshcomponents false false)
  (`PrimitiveComponent.SetCollisionEnabled` _meshcomponents "NoCollision")
  (`PrimitiveComponent.SetCollisionEnabled` (`self.BoxCollisionList`) "NoCollision")
  (`SceneComponent.SetVisibility` _item true false)
  (`PrimitiveComponent.SetCollisionEnabled` _item "QueryAndPhysics")
  (if (`self.GenerateBoxCollision`)
    (`PrimitiveComponent.SetCollisionEnabled` (`KismetArrayLibrary.Array_Get` (`self.BoxCollisionList`) (`self.MeshIndex`)) "QueryAndPhysics"))
  ;[1 1 1] Check if Base Mesh is Selected
  (if (== (`self.MeshIndex`) 0)
    ;[1 1 1] Set Overriden Base Materials
    (for (_array_element _array_index) (`self.BaseMaterials`)
      (`PrimitiveComponent.SetMaterial` _item _array_index _array_element))
    ;[1 1 1] Set Non Overriden Base Materials
    (for (_array_element_2 _array_index_2) (`self.BaseMeshMaterials`)
      (if (not (<= _array_index_2 (`KismetArrayLibrary.Array_LastIndex` (`self.BaseMaterials`))))
        (`PrimitiveComponent.SetMaterial` _item _array_index_2 _array_element_2)))
    (elif (== (`KismetArrayLibrary.Array_Length` _materialoverrides) 0)
      (`/Engine/EditorBlueprintResources/StandardMacros.IsValid` _meshoverride
        (:`Is Valid`
          _)
        (:`Is Not Valid`
          ;[1 1 1] Set to Default Material if No Overrides Provided
          (`PrimitiveComponent.SetMaterial` _item_2 0 (`KismetArrayLibrary.Array_Get` _returnvalue))))
      (else
        (for (_array_element_3 _array_index_3) _materialoverrides
          ;[1 1 1] Set Object Material
          (`/Engine/EditorBlueprintResources/StandardMacros.IsValid` _array_element_3
            (:`Is Valid`
              (`PrimitiveComponent.SetMaterial` _item_2 _array_index_3 _array_element_3))
            (:`Is Not Valid`
              (`PrimitiveComponent.SetMaterial` _item_2 _array_index_3 (select `bool` (`KismetSystemLibrary.IsValid` _meshoverride) :`false` (`KismetArrayLibrary.Array_Get` (`self.BaseMaterials`) _array_index_3) :`true` (`KismetArrayLibrary.Array_Get` _returnvalue _array_index_3)))))))))
  ;[1 1 1] Enable or Disable Collision
  (if (`self.EnableCollision`)
    (`PrimitiveComponent.SetCollisionResponseToChannel` _item "ECC_Pawn" "ECR_Block")
    (else
      (`PrimitiveComponent.SetCollisionResponseToChannel` _item "ECC_Pawn" "ECR_Overlap")))
  ;[1 1 1] Set Shadow Mesh
  (`StaticMeshComponent.SetStaticMesh` _shadowmesh (`KismetArrayLibrary.Array_Get` (`self.Meshes`) _meshindex))
  (`SceneComponent.SetVisibility` _shadowmesh false false)
  (`PrimitiveComponent.SetRenderCustomDepth` _item true))

(fn `UserConstructionScript`
  (bind _shadowmesh (`self.ShadowMesh`))
  (bind _basemeshcomponent (`self.BaseMeshComponent`))
  (bind _boxcollisionlist (`self.BoxCollisionList`))
  ;[1 1 1] Check If Render Stage Exists
  (bind _outactors (`GameplayStatics.GetAllActorsOfClass` "/Game/HALArchvizToolkit/Blueprints/BP_ThumbnailRenderStage.BP_ThumbnailRenderStage_C"))
  (if (>= (`KismetArrayLibrary.Array_LastIndex` _outactors) 0)
    (set `self.RenderStageExists` true)
    (else
      (set `self.RenderStageExists` false)))
  (set `self.MeshOverride` false)
  (`KismetArrayLibrary.Array_Clear` (`self.Meshes`))
  (`KismetArrayLibrary.Array_Clear` (`self.MeshComponents`))
  (`/Engine/EditorBlueprintResources/StandardMacros.IsValid` (`self.BaseMesh`)
    (:`Is Valid`
      ;[1 1 1] Check if Switching Meshes
      (for _array_element (`self.SwitchingOptions`)
        (`/Engine/EditorBlueprintResources/StandardMacros.IsValid` (`.MeshOverride_38_11DD1DC340A51933F3FBBA8636E3E738` (break `/Game/HALArchvizToolkit/Blueprints/ObjectChoices` _array_element))
          (:`Is Valid`
            (set `self.MeshOverride` true)
            (break))))
      (if (`self.MeshOverride`)
        ;[1 1 1] Only Self Shadow if Switching Meshes
        (bind _returnvalue (`AddComponent|StaticMeshComponent_1341`))
        (else
          ;[1 1 1] Add Initial Base Mesh
          (bind _returnvalue_2 (`AddComponent|StaticMeshComponent_187`))))
      (bind _returnvalue_3 (select `bool` (`self.MeshOverride`) :`false` _returnvalue_2 :`true` _returnvalue))
      (`StaticMeshComponent.SetStaticMesh` _returnvalue_3 (`self.BaseMesh`))
      ;[1 1 1] Set Base Materials
      (set `self.BaseMeshMaterials` (`MeshComponent.GetMaterials` _returnvalue_3))
      (for (_array_element_2 _array_index) (`self.BaseMaterials`)
        (`PrimitiveComponent.SetMaterial` _returnvalue_3 _array_index _array_element_2))
      (bind _output_get (set `self.BaseMeshComponent` _returnvalue_3))
      (`KismetArrayLibrary.Array_Add` (`self.MeshComponents`) _output_get)
      (`KismetArrayLibrary.Array_Add` (`self.Meshes`) (`self.BaseMesh`))
      (for (_array_element_3 _array_index_2) (`self.SwitchingOptions`)
        (bind (_meshoverride _materialoverrides) (break `/Game/HALArchvizToolkit/Blueprints/ObjectChoices` _array_element_3))
        (`/Engine/EditorBlueprintResources/StandardMacros.IsValid` _meshoverride
          (:`Is Valid`
            ;[1 1 1] Add Mesh Override
            (bind _returnvalue_4 (`AddComponent|StaticMeshComponent_188`))
            (`StaticMeshComponent.SetStaticMesh` _returnvalue_4 _meshoverride)
            (`KismetArrayLibrary.Array_Add` (`self.MeshComponents`) _returnvalue_4)
            (`KismetArrayLibrary.Array_Add` (`self.Meshes`) _meshoverride)
            (for (_array_element_4 _array_index_3) _materialoverrides
              (`PrimitiveComponent.SetMaterial` _returnvalue_4 _array_index_3 _array_element_4))
            ;[1 1 1] Disable Visibility and Collision for Override Meshes
            (`SceneComponent.SetVisibility` _returnvalue_4 false false)
            (`PrimitiveComponent.SetCollisionEnabled` _returnvalue_4 "NoCollision"))
          (:`Is Not Valid`
            ;[1 1 1] Add Reference to Base Mesh if No Override is Provided
            (`KismetArrayLibrary.Array_Add` (`self.MeshComponents`) (`self.BaseMeshComponent`))
            (`KismetArrayLibrary.Array_Add` (`self.Meshes`) (`self.BaseMesh`))))
        (if (`self.GenerateBoxCollision`)
          (bind _item (`KismetArrayLibrary.Array_Get` (`self.MeshComponents`) _array_index_2))
          (bind (_origin _boxextent) (`KismetSystemLibrary.GetComponentBounds` _item))
          ;[1 1 1] Generate Box Collision
          (bind _returnvalue_5 (`AddComponent|Box Collision_3` :`RelativeTransform` (`KismetMathLibrary.MakeTransform` (`KismetMathLibrary.InverseTransformLocation` (`SceneComponent.K2_GetComponentToWorld` _item) _origin))))
          (`KismetArrayLibrary.Array_Add` (`self.BoxCollisionList`) _returnvalue_5)
          (`PrimitiveComponent.SetCollisionEnabled` _returnvalue_5 "NoCollision")
          (`BoxComponent.SetBoxExtent` _returnvalue_5 _boxextent true)
          ;[1 1 1] Check if Collision is Enabled for Box
          (if (`self.EnableCollision`)
            (`PrimitiveComponent.SetCollisionResponseToChannel` _returnvalue_5 "ECC_Pawn" "ECR_Block")
            (else
              (`PrimitiveComponent.SetCollisionResponseToChannel` _returnvalue_5 "ECC_Pawn" "ECR_Overlap")))
          (if (>= (`KismetArrayLibrary.Array_LastIndex` _boxcollisionlist) 0)
            ;[1 1 1] Enable Collision for Base Mesh
            (`PrimitiveComponent.SetCollisionEnabled` (`KismetArrayLibrary.Array_Get` _boxcollisionlist) "QueryAndPhysics"))))
      ;[1 1 1] Set Initial Shadow Mesh
      (`StaticMeshComponent.SetStaticMesh` _shadowmesh (`KismetArrayLibrary.Array_Get` (`self.Meshes`)))
      (`SceneComponent.SetVisibility` _shadowmesh false false)
      ;[1 1 1] Check if Collision is Enabled for Mesh
      (if (`self.EnableCollision`)
        (`PrimitiveComponent.SetCollisionResponseToChannel` _basemeshcomponent "ECC_Pawn" "ECR_Block")
        (else
          (`PrimitiveComponent.SetCollisionResponseToChannel` _basemeshcomponent "ECC_Pawn" "ECR_Overlap"))))))