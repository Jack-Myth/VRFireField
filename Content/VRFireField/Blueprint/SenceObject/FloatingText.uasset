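; FloatingText is an actor that displays text in the world through a ClickableButton user widget on its widget component.
; BeginPlay and the SetText event both push TextToShow into the widget, then destroy the actor after DelayToDestroy when that value is non-zero.
; FollowPlayer enables Tick, which turns the actor on yaw alone to face the first player's pawn.
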(event `SetText`
  (params (NewText :type Text))
  (bind _delaytodestroy (`self.DelayToDestroy`))
  (set `self.TextToShow` NewText)
  (bind _asclickable_button (cast `/Game/VRFireField/Blueprint/BaseObject/ClickableButton` (`WidgetComponent.GetUserWidgetObject` (`self.Widget`)) :!label _label))
  (`/Game/VRFireField/Blueprint/BaseObject/ClickableButton.SetText` _asclickable_button (`self.TextToShow`))
  (if (!= _delaytodestroy 0.0)
    (`KismetSystemLibrary.Delay` _delaytodestroy)
    (`self.K2_DestroyActor`)))

(event `self.ReceiveBeginPlay`
  (if (`self.FollowPlayer`)
    (`self.SetActorTickEnabled` true)
    (goto _label)
    (else
      (goto _label))))

(event `self.ReceiveTick`
  (params (DeltaSeconds :type "Float (single-precision)"))
  (bind (_returnvalue_roll _returnvalue_pitch _returnvalue_yaw) (`KismetMathLibrary.BreakRotator` (`KismetMathLibrary.FindLookAtRotation` (`self.K2_GetActorLocation`) (`self.K2_GetActorLocation` (`GameplayStatics.GetPlayerPawn` 0)))))
  (`self.K2_SetActorRotation` (`KismetMathLibrary.MakeRotator` 0.0 0.0 _returnvalue_yaw)))

(fn `UserConstructionScript`)