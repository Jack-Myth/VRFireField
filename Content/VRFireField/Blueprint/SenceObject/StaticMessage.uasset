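; StaticMessage is a scene actor that shows a text message when a character comes near it.
; On BeginPlay it writes its Message variable into a Text2D user widget on its Widget component, then hides the whole actor.
; Sphere overlap events unhide the actor when a Character enters and hide it again when one leaves.
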(event `self.Sphere.OnComponentBeginOverlap`
  (params (OverlappedComponent :type "PrimitiveComponent Object Reference") (OtherActor :type "Actor Object Reference") (OtherComp :type "PrimitiveComponent Object Reference") (OtherBodyIndex :type Integer) (bFromSweep :type Boolean) (SweepResult :type "HitResult Structure (by ref)"))
  (cast `Character` OtherActor)
  (`self.SetActorHiddenInGame` false))

(event `self.ReceiveBeginPlay`
  (bind _astext_2d (cast `/Game/VRFireField/Blueprint/BaseObject/Text2D` (`WidgetComponent.GetUserWidgetObject` (`self.Widget`))))
  (`/Game/VRFireField/Blueprint/BaseObject/Text2D.SetText` _astext_2d (`self.Message`))
  (`self.SetActorHiddenInGame` true))

(event `self.Sphere.OnComponentEndOverlap`
  (params (OverlappedComponent :type "PrimitiveComponent Object Reference") (OtherActor :type "Actor Object Reference") (OtherComp :type "PrimitiveComponent Object Reference") (OtherBodyIndex :type Integer))
  (cast `Character` OtherActor)
  (`self.SetActorHiddenInGame` true))

(fn `UserConstructionScript`)