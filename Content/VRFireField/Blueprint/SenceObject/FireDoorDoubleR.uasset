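; VR-grabbable hinged fire door, apparently the right leaf of a double door.
; While held, Tick yaws the mesh toward the hand within ±90 degrees of the actor's facing.
; On release, timelines ease it shut or fully open depending on angle, re-snapping the grab sphere to its anchor.
; CloseDoor and OpenDoor events reuse this timeline-lerp approach, and dispatchers report opened, closed and mesh overlap.
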(event `self.BeginCatch`
  (params (HoldingHand :type "PrimitiveComponent Object Reference"))
  (`parent.BeginCatch` HoldingHand)
  (if (`self.CanBeOpend`)
    (set `self.HoldingHands` HoldingHand)
    (`self.SetActorTickEnabled` true)
    (set `self.IsDoorOpend` false)
    (set `self.IsDoorClosed` false)
    (bind (_direction `_新建轨迹_0`) (`Timeline|时间轴_0` :!via `Stop` :!label _label)
      (:`Update`
        (`SceneComponent.K2_SetRelativeRotation` (`self.StaticMesh`) (`KismetMathLibrary.MakeRotator` 0.0 0.0 (`KismetMathLibrary.Lerp` (stale `self.EndCatch` _output_get) 0.0 `_新建轨迹_0`)) false false)
        (`SceneComponent.K2_SetWorldLocation` (`self.Sphere_Catch`) (`SceneComponent.K2_GetComponentLocation` (`self.Scene`)) false false))
      (:`Finished`
        (set `self.IsDoorClosed` true)
        (set `self.IsDoorOpend` false)
        (`self.DoorClosed`)))))

(event `self.EndCatch`
  (params (LastHoldHand :type "PrimitiveComponent Object Reference"))
  (bind _staticmesh (`self.StaticMesh`))
  (bind _returnvalue (`SceneComponent.GetRelativeTransform` _staticmesh))
  (`parent.EndCatch` LastHoldHand)
  (`self.SetActorTickEnabled` false)
  (if (< (`KismetMathLibrary.Abs` (.yaw (.rotation _returnvalue))) 30.0)
    (bind _output_get (set `self.TmpYaw` (.yaw (.rotation _returnvalue)) :!label _label_2))
    (goto _label :!via `PlayFromStart`)
    (else
      (bind _output_get_2 (set `self.TmpYaw` (.yaw (.rotation _returnvalue))))
      (bind (_direction `_新建轨迹_0`) (`Timeline|时间轴_1` :!via `PlayFromStart`)
        (:`Update`
          (`SceneComponent.K2_SetRelativeRotation` _staticmesh (`KismetMathLibrary.MakeRotator` 0.0 0.0 (`KismetMathLibrary.Lerp` _output_get_2 (* 90 (/ (.yaw (.rotation _returnvalue)) (`KismetMathLibrary.Abs` (.yaw (.rotation _returnvalue))))) `_新建轨迹_0`)) false false)
          (`SceneComponent.K2_SetWorldLocation` (`self.Sphere_Catch`) (`SceneComponent.K2_GetComponentLocation` (`self.Scene`)) false false))
        (:`Finished`
          (set `self.IsDoorClosed` false)
          (set `self.IsDoorOpend` true)
          (`self.DoorOpend`))))))

(event `self.CloseDoor`
  (goto _label_2))

(event `self.ReceiveTick`
  (params (DeltaSeconds :type "Float (single-precision)"))
  (bind (_returnvalue_roll _returnvalue_pitch _returnvalue_yaw) (`KismetMathLibrary.BreakRotator` (`self.K2_GetActorRotation`)))
  (bind (_returnvalue_roll_2 _returnvalue_pitch_2 _returnvalue_yaw_2) (`KismetMathLibrary.BreakRotator` (`KismetMathLibrary.FindLookAtRotation` (`SceneComponent.K2_GetComponentLocation` (`self.StaticMesh`)) (`SceneComponent.K2_GetComponentLocation` (`self.HoldingHands`)))))
  (bind _standardrotator (`/Game/MacroLibrary.StandardRotator` (`KismetMathLibrary.MakeRotator` 0.0 0.0 (- _returnvalue_yaw_2 _returnvalue_yaw))))
  (if (not (or (> (.yaw _standardrotator) 90.0) (< (.yaw _standardrotator) -90.0)))
    (`SceneComponent.K2_SetWorldRotation` (`self.StaticMesh`) (`KismetMathLibrary.MakeRotator` 0.0 0.0 _returnvalue_yaw_2) false false)))

(event `self.OpenDoor`
  (`self.OpenDoorWithDir` 90.0))

(event `self.StaticMesh.OnComponentBeginOverlap`
  (params (OverlappedComponent :type "PrimitiveComponent Object Reference") (OtherActor :type "Actor Object Reference") (OtherComp :type "PrimitiveComponent Object Reference") (OtherBodyIndex :type Integer) (bFromSweep :type Boolean) (SweepResult :type "HitResult Structure (by ref)"))
  (`self.Overlap` OtherActor OtherComp))

(event `OpenDoorWithDir`
  (params (Dir :type "Float (double-precision)"))
  (bind _staticmesh (`self.StaticMesh`))
  (bind _output_get (set `self.TmpYaw` (.yaw (.rotation (`SceneComponent.GetRelativeTransform` _staticmesh)))))
  (bind (_direction `_新建轨迹_0`) (`Timeline|时间轴_2` :!via `PlayFromStart`)
    (:`Update`
      (`SceneComponent.K2_SetRelativeRotation` _staticmesh (`KismetMathLibrary.MakeRotator` 0.0 0.0 (`KismetMathLibrary.Lerp` _output_get Dir `_新建轨迹_0`)) false false)
      (`SceneComponent.K2_SetWorldLocation` (`self.Sphere_Catch`) (`SceneComponent.K2_GetComponentLocation` (`self.Scene`)) false false))
    (:`Finished`
      (set `self.IsDoorOpend` true)
      (set `self.IsDoorClosed` false)
      (`self.DoorOpend`))))

(fn `UserConstructionScript`)