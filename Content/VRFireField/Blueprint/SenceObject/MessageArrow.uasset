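; MessageArrow is a floor or guide arrow sprite that marks a spot and reacts when a character steps on it.
; A timeline started on BeginPlay slides the paper sprite back and forth along its local X axis.
; When a Character overlaps the visible sprite, it fires a WalkOn call and destroys itself if DestoryWhenStepOn is set.
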(event `self.ReceiveBeginPlay`
  (bind (_direction `_新建轨迹_0`) (`Timeline|时间轴_0`)
    (:`Update`
      (`SceneComponent.K2_SetRelativeLocation` (`self.PaperSprite`) (`KismetMathLibrary.VLerp` (-10.0 0.0 0.02) (10.0 0.0 0.02) `_新建轨迹_0`) false false))))

(event `self.PaperSprite.OnComponentBeginOverlap`
  (params (OverlappedComponent :type "PrimitiveComponent Object Reference") (OtherActor :type "Actor Object Reference") (OtherComp :type "PrimitiveComponent Object Reference") (OtherBodyIndex :type Integer) (bFromSweep :type Boolean) (SweepResult :type "HitResult Structure (by ref)"))
  (if (not (`self.bHidden`))
    (cast `Character` OtherActor)
    (`self.WalkOn` self)
    (if (`self.DestoryWhenStepOn`)
      (`self.K2_DestroyActor`))))

(fn `UserConstructionScript`)