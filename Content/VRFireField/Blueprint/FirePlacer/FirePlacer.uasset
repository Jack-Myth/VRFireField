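; FirePlacer is a VR pawn with camera-yaw-relative movement that places objects using a right motion controller laser pointer.
; Each tick, a visibility trace scales the cursor beam and sends select begin/end messages as the hit component changes.
; The action button sends tele-click messages on widgets or placeable meshes, otherwise spawning the indexed object at the hit point.
; The menu button alternately spawns the menu and closes it with its sub-panels.
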(event `self.ReceiveTick`
  (params (DeltaSeconds :type "Float (single-precision)"))
  (bind _cylinder_vrcursor (`self.Cylinder_VRCursor`))
  (bind _motioncontroller_r (`self.MotionController_R`))
  (bind _currentselectcomponent (`self.CurrentSelectComponent`))
  (bind _returnvalue (`SceneComponent.K2_GetComponentLocation` _motioncontroller_r))
  (bind (_outhit _returnvalue_2) (`KismetSystemLibrary.LineTraceSingle` :`Start` _returnvalue :`End` (+ _returnvalue (* (`SceneComponent.GetForwardVector` _motioncontroller_r) 99999)) :`TraceChannel` "TraceTypeQuery1" :`DrawDebugType` "ForOneFrame"))
  (if _returnvalue_2
    (bind (_bblockinghit _binitialoverlap _time _location _impactpoint _normal _impactnormal _physmat _hitactor _hitcomponent) (`GameplayStatics.BreakHitResult` _outhit))
    (`SceneComponent.SetWorldScale3D` _cylinder_vrcursor (`KismetMathLibrary.MakeVector` 1.0 1.0 (`KismetMathLibrary.VSize` (/ (- _location _returnvalue) 100))))
    (if (!= _hitcomponent _currentselectcomponent)
      (`/Engine/EditorBlueprintResources/StandardMacros.IsValid` _currentselectcomponent
        (:`Is Valid`
          (message `/Game/VRFireField/Blueprint/BaseObject/MotionInterface.EndSelect` (`ActorComponent.GetOwner` _currentselectcomponent) _currentselectcomponent))
        (:`Is Not Valid`
          _))
      (bind _output_get (set `self.CurrentSelectComponent` _hitcomponent))
      (message `/Game/VRFireField/Blueprint/BaseObject/MotionInterface.BeginSelect` (`ActorComponent.GetOwner` _output_get) (`self.CurrentSelectComponent`)))
    (else
      (`SceneComponent.SetWorldScale3D` _cylinder_vrcursor (1.0 1.0 99999.0))
      (set `self.CurrentSelectComponent` null))))

(event `InputAxis|MoveForword`
  (params (AxisValue :type "Float (single-precision)"))
  (bind (_returnvalue_roll _returnvalue_pitch _returnvalue_yaw) (`KismetMathLibrary.BreakRotator` (`SceneComponent.K2_GetComponentRotation` (`self.Camera`))))
  (`self.AddMovementInput` (`KismetMathLibrary.GetForwardVector` (`KismetMathLibrary.MakeRotator` 0.0 0.0 _returnvalue_yaw)) (/ AxisValue 2.0)))

(event `InputAxis|ViewX`
  (params (AxisValue :type "Float (single-precision)"))
  (`self.AddControllerYawInput` AxisValue))

(event `InputAxis|MoveRight`
  (params (AxisValue :type "Float (single-precision)"))
  (bind (_returnvalue_roll _returnvalue_pitch _returnvalue_yaw) (`KismetMathLibrary.BreakRotator` (`SceneComponent.K2_GetComponentRotation` (`self.Camera`))))
  (`self.AddMovementInput` (`KismetMathLibrary.GetRightVector` (`KismetMathLibrary.MakeRotator` 0.0 0.0 _returnvalue_yaw)) (/ AxisValue 2.0)))

(event `InputAxis|ViewY`
  (params (AxisValue :type "Float (single-precision)"))
  (`self.AddControllerPitchInput` AxisValue))

(event `InputAction|Menu`
  (params (Key :type "Key Structure" :default "AnyKey"))
  (bind _motioncontroller_r (`self.MotionController_R`))
  (:`Pressed`
    (`/Engine/EditorBlueprintResources/StandardMacros.FlipFlop`
      (:`A`
        (`|SpawnActorFromClass` "/Game/VRFireField/Blueprint/FirePlacer/Menu.Menu_C" (`KismetMathLibrary.MakeTransform` (+ (+ (`SceneComponent.K2_GetComponentLocation` _motioncontroller_r) (* (`SceneComponent.GetForwardVector` _motioncontroller_r) 100)) (0.0 0.0 70.0)) (struct) (0.5 0.5 0.5)) "Undefined" "OverrideRootScale"))
      (:`B`
        (bind _outactors (`GameplayStatics.GetAllActorsOfClass` "/Game/VRFireField/Blueprint/FirePlacer/Menu.Menu_C"))
        (for _array_element _outactors
          (`/Game/VRFireField/Blueprint/FirePlacer/Menu.CloseMenu` _array_element))
        (bind _outactors_2 (`GameplayStatics.GetAllActorsOfClass` "/Game/VRFireField/Blueprint/FirePlacer/Keyboard.Keyboard_C"))
        (`self.K2_DestroyActor` _outactors_2)
        (bind _outactors_3 (`GameplayStatics.GetAllActorsOfClass` "/Game/VRFireField/Blueprint/FirePlacer/SelectPlaceableObject.SelectPlaceableObject_C"))
        (`self.K2_DestroyActor` _outactors_3)
        (bind _outactors_4 (`GameplayStatics.GetAllActorsOfClass` "/Game/VRFireField/Blueprint/FirePlacer/Load.Load_C"))
        (`self.K2_DestroyActor` _outactors_4)))))

(event `InputAction|ActionForR`
  (params (Key :type "Key Structure" :default "AnyKey"))
  (bind _currentselectcomponent (`self.CurrentSelectComponent`))
  (bind _motioncontroller_r (`self.MotionController_R`))
  (bind _returnvalue (`SceneComponent.K2_GetComponentLocation` _motioncontroller_r))
  (bind _returnvalue_2 (`ActorComponent.GetOwner` _currentselectcomponent))
  (:`Pressed`
    (bind (_outhit _returnvalue_3) (`KismetSystemLibrary.LineTraceSingle` _returnvalue (+ _returnvalue (* (`SceneComponent.GetForwardVector` _motioncontroller_r) 99999)) "TraceTypeQuery1"))
    (if _returnvalue_3
      (bind (_bblockinghit _binitialoverlap _time _location _impactpoint _normal _impactnormal _physmat _hitactor _hitcomponent) (`GameplayStatics.BreakHitResult` _outhit))
      (cast `WidgetComponent` _hitcomponent
        (:`then`
          (message `/Game/VRFireField/Blueprint/BaseObject/MotionInterface.BeginTeleClick` _returnvalue_2 _currentselectcomponent :!label _label))
        (:`CastFailed`
          (cast `/Game/VRFireField/Blueprint/BaseObject/PlaceableMeshActor` _hitactor
            (:`then`
              (goto _label))
            (:`CastFailed`
              (`|SpawnActorFromClass` (`KismetArrayLibrary.Array_Get` (`self.ObjectItem`) (`self.ObjectIndex`)) (`KismetMathLibrary.MakeTransform` _location) "Undefined" "OverrideRootScale")
              (set `self.CurrentPlaceableMesh` null)))))))
  (:`Released`
    (message `/Game/VRFireField/Blueprint/BaseObject/MotionInterface.EndTeleClick` _returnvalue_2 _currentselectcomponent)))

(fn `UserConstructionScript`)