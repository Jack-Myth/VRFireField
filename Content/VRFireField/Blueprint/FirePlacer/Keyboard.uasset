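; In-world VR keyboard actor whose keys are KeyboardButton widgets on WidgetComponents, used to edit a supplied text target.
; INIT hands that EditableText to every button, then labels A to Z by finding each component through its matching letter tag.
; Select, deselect and tele-click events resolve the hit component to its button widget and forward the call.
; Tick turns the actor's yaw to face the player pawn.
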(event `INIT`
  (params (EditableText :type "EditableTextBox Object Reference"))
  ;[1 1 1] INIT
  (for _array_element (`self.K2_GetComponentsByClass` "/Script/UMG.WidgetComponent")
    (bind _askeyboard_button (cast `/Game/VRFireField/Blueprint/BaseObject/KeyboardButton` (`WidgetComponent.GetUserWidgetObject` _array_element)))
    (set `/Game/VRFireField/Blueprint/BaseObject/KeyboardButton.EditText` EditableText _askeyboard_button))
  (`self.SetText` "A"
    (:`Out`
      (`self.SetText` "B"
        (:`Out`
          (`self.SetText` "C"
            (:`Out`
              (`self.SetText` "D"
                (:`Out`
                  (`self.SetText` "E"
                    (:`Out`
                      (`self.SetText` "F"
                        (:`Out`
                          (`self.SetText` "G"
                            (:`Out`
                              (`self.SetText` "H"
                                (:`Out`
                                  (`self.SetText` "I"
                                    (:`Out`
                                      (`self.SetText` "J"
                                        (:`Out`
                                          (`self.SetText` "K"
                                            (:`Out`
                                              (`self.SetText` "L"
                                                (:`Out`
                                                  (`self.SetText` "M"
                                                    (:`Out`
                                                      (`self.SetText` "N"
                                                        (:`Out`
                                                          (`self.SetText` "O"
                                                            (:`Out`
                                                              (`self.SetText` "P"
                                                                (:`Out`
                                                                  (`self.SetText` "Q"
                                                                    (:`Out`
                                                                      (`self.SetText` "R"
                                                                        (:`Out`
                                                                          (`self.SetText` "S"
                                                                            (:`Out`
                                                                              (`self.SetText` "T"
                                                                                (:`Out`
                                                                                  (`self.SetText` "U"
                                                                                    (:`Out`
                                                                                      (`self.SetText` "V"
                                                                                        (:`Out`
                                                                                          (`self.SetText` "W"
                                                                                            (:`Out`
                                                                                              (`self.SetText` "X"
                                                                                                (:`Out`
                                                                                                  (`self.SetText` "Y"
                                                                                                    (:`Out`
                                                                                                      (`self.SetText` "Z"))))))))))))))))))))))))))))))))))))))))))))))))))))

(event `/Game/VRFireField/Blueprint/BaseObject/MotionInterface.BeginSelect`
  (params (SelectedComponent :type "PrimitiveComponent Object Reference"))
  ;[1 1 1] 事件调用
  (bind _keyboardbutton (`self.FindWidget` SelectedComponent)
    (:`Out`
      (`/Game/VRFireField/Blueprint/BaseObject/KeyboardButton.BeginSelect` _keyboardbutton))))

(event `/Game/VRFireField/Blueprint/BaseObject/MotionInterface.BeginTeleClick`
  (params (ClickTargetComponent :type "PrimitiveComponent Object Reference"))
  ;[1 1 1] 事件调用
  (bind _keyboardbutton (`self.FindWidget` ClickTargetComponent)
    (:`Out`
      (`/Game/VRFireField/Blueprint/BaseObject/KeyboardButton.BeginClick` _keyboardbutton))))

(event `/Game/VRFireField/Blueprint/BaseObject/MotionInterface.EndSelect`
  (params (LastSelectedComponent :type "PrimitiveComponent Object Reference"))
  ;[1 1 1] 事件调用
  (bind _keyboardbutton (`self.FindWidget` LastSelectedComponent)
    (:`Out`
      (`/Game/VRFireField/Blueprint/BaseObject/KeyboardButton.EndSelect` _keyboardbutton))))

(event `self.ReceiveTick`
  (params (DeltaSeconds :type "Float (single-precision)"))
  (bind (_returnvalue_roll _returnvalue_pitch _returnvalue_yaw) (`KismetMathLibrary.BreakRotator` (`KismetMathLibrary.FindLookAtRotation` (`self.K2_GetActorLocation`) (`self.K2_GetActorLocation` (`GameplayStatics.GetPlayerPawn` 0)))))
  (`self.K2_SetActorRotation` (`KismetMathLibrary.MakeRotator` 0.0 0.0 _returnvalue_yaw)))

(fn `UserConstructionScript`)