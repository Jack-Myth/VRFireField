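; World-space VR menu actor in the fire placer, with buttons for selecting objects, saving or loading the scene, returning to the main menu and starting play.
; Each option spawns its submenu, opens MainMenu or possesses a new FireFighter, then reverses the opening timeline and destroys the menu.
; Pointer select and click events resolve widget components to ClickableButtons through FindWidget.
; Tick keeps the menu yawed toward the player.
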(event `/Game/VRFireField/Blueprint/BaseObject/MotionInterface.BeginSelect`
  (params (SelectedComponent :type "PrimitiveComponent Object Reference"))
  ;[1 1 1] 事件调用
  (bind _clickablebutton (`self.FindWidget` SelectedComponent)
    (:`Out`
      (`/Game/VRFireField/Blueprint/BaseObject/ClickableButton.BeginSelect` _clickablebutton))))

(event `CloseMenu`
  ;[1 1 1] INIT
  (bind (_direction _1 _2 _3 _4) (`Timeline|TimeLineForMenuOpen` :!via `Reverse` :!label _label)
    (:`Update`
      (`SceneComponent.K2_SetRelativeLocation` (`self.Save`) (`KismetMathLibrary.MakeVector` 0.0 0.0 _1) false false)
      (`SceneComponent.K2_SetRelativeLocation` (`self.Load`) (`KismetMathLibrary.MakeVector` 0.0 0.0 _2) false false)
      (`SceneComponent.K2_SetRelativeLocation` (`self.Back`) (`KismetMathLibrary.MakeVector` 0.0 0.0 _3) false false)
      (`SceneComponent.K2_SetRelativeLocation` (`self.Play`) (`KismetMathLibrary.MakeVector` 0.0 0.0 _4) false false))
    (:`Finished`
      (if (`|EnumEquality` _direction "Backward")
        (`self.K2_DestroyActor`)))))

(event `self.ReceiveBeginPlay`
  (bind _asclickable_button (cast `/Game/VRFireField/Blueprint/BaseObject/ClickableButton` (`WidgetComponent.GetUserWidgetObject` (`self.Play`)) :!pure true))
  (bind _asclickable_button_2 (cast `/Game/VRFireField/Blueprint/BaseObject/ClickableButton` (`WidgetComponent.GetUserWidgetObject` (`self.Back`)) :!pure true))
  (bind _asclickable_button_3 (cast `/Game/VRFireField/Blueprint/BaseObject/ClickableButton` (`WidgetComponent.GetUserWidgetObject` (`self.SelectObject`)) :!pure true))
  (bind _asclickable_button_4 (cast `/Game/VRFireField/Blueprint/BaseObject/ClickableButton` (`WidgetComponent.GetUserWidgetObject` (`self.Save`)) :!pure true))
  (bind _asclickable_button_5 (cast `/Game/VRFireField/Blueprint/BaseObject/ClickableButton` (`WidgetComponent.GetUserWidgetObject` (`self.Load`)) :!pure true))
  ;[1 1 1] INIT
  (`/Game/VRFireField/Blueprint/BaseObject/ClickableButton.SetText` _asclickable_button_3 "选择物件")
  (add `/Game/VRFireField/Blueprint/BaseObject/ClickableButton.BeginClick` _asclickable_button_3 (delegate `OpenMenuForSelect`))
  (`/Game/VRFireField/Blueprint/BaseObject/ClickableButton.SetText` _asclickable_button_4 "保存场景")
  (add `/Game/VRFireField/Blueprint/BaseObject/ClickableButton.BeginClick` _asclickable_button_4 (delegate `OpenMenuForSave`))
  (`/Game/VRFireField/Blueprint/BaseObject/ClickableButton.SetText` _asclickable_button_5 "读取场景")
  (add `/Game/VRFireField/Blueprint/BaseObject/ClickableButton.BeginClick` _asclickable_button_5 (delegate `OpenMenuForLoad`))
  (`/Game/VRFireField/Blueprint/BaseObject/ClickableButton.SetText` _asclickable_button_2 "返回")
  (add `/Game/VRFireField/Blueprint/BaseObject/ClickableButton.BeginClick` _asclickable_button_2 (delegate `BackUpward`))
  (`/Game/VRFireField/Blueprint/BaseObject/ClickableButton.SetText` _asclickable_button "开始")
  (add `/Game/VRFireField/Blueprint/BaseObject/ClickableButton.BeginClick` _asclickable_button (delegate `StartPlay`))
  (goto _label))

(event `/Game/VRFireField/Blueprint/BaseObject/MotionInterface.BeginTeleClick`
  (params (ClickTargetComponent :type "PrimitiveComponent Object Reference"))
  ;[1 1 1] 事件调用
  (bind _clickablebutton (`self.FindWidget` ClickTargetComponent)
    (:`Out`
      (`/Game/VRFireField/Blueprint/BaseObject/ClickableButton.BeginClick` _clickablebutton))))

(event `OpenMenuForSelect`
  ;[1 1 1] INIT
  (`|SpawnActorFromClass` "/Game/VRFireField/Blueprint/FirePlacer/SelectPlaceableObject.SelectPlaceableObject_C" (`KismetMathLibrary.MakeTransform` (- (`self.K2_GetActorLocation`) (0.0 0.0 40.0)) (struct)) "Undefined" "OverrideRootScale")
  (`self.CloseMenu`))

(event `/Game/VRFireField/Blueprint/BaseObject/MotionInterface.EndSelect`
  (params (LastSelectedComponent :type "PrimitiveComponent Object Reference"))
  ;[1 1 1] 事件调用
  (bind _clickablebutton (`self.FindWidget` LastSelectedComponent)
    (:`Out`
      (`/Game/VRFireField/Blueprint/BaseObject/ClickableButton.EndSelect` _clickablebutton))))

(event `OpenMenuForSave`
  ;[1 1 1] INIT
  (`|SpawnActorFromClass` "/Game/VRFireField/Blueprint/FirePlacer/Save.Save_C" (`KismetMathLibrary.MakeTransform` (`self.K2_GetActorLocation`) (struct)) "Undefined" "OverrideRootScale")
  (`self.CloseMenu`))

(event `self.ReceiveTick`
  (params (DeltaSeconds :type "Float (single-precision)"))
  (bind (_returnvalue_roll _returnvalue_pitch _returnvalue_yaw) (`KismetMathLibrary.BreakRotator` (`KismetMathLibrary.FindLookAtRotation` (`self.K2_GetActorLocation`) (`self.K2_GetActorLocation` (`GameplayStatics.GetPlayerPawn` 0)))))
  (`self.K2_SetActorRotation` (`KismetMathLibrary.MakeRotator` 0.0 0.0 _returnvalue_yaw)))

(event `OpenMenuForLoad`
  ;[1 1 1] INIT
  (`|SpawnActorFromClass` "/Game/VRFireField/Blueprint/FirePlacer/Load.Load_C" (`KismetMathLibrary.MakeTransform` (`self.K2_GetActorLocation`) (struct)) "Undefined" "OverrideRootScale")
  (`self.CloseMenu`))

(event `BackUpward`
  ;[1 1 1] INIT
  (`self.CloseMenu`)
  (`GameplayStatics.OpenLevel` "MainMenu"))

(event `StartPlay`
  (bind _returnvalue (`GameplayStatics.GetPlayerPawn` 0))
  ;[1 1 1] INIT
  (bind _returnvalue_2 (`|SpawnActorFromClass` "/Game/VRFireField/Blueprint/FireFighter.FireFighter_C" (`self.GetTransform` _returnvalue) "AlwaysSpawn" "OverrideRootScale"))
  (`self.K2_DestroyActor` _returnvalue)
  (`Controller.Possess` (`GameplayStatics.GetPlayerController` 0) _returnvalue_2)
  (`self.CloseMenu`))

(fn `UserConstructionScript`)