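; SelectPlaceableObject is an in-world widget panel for stepping between placeable objects in the VR fire-field placer.
; On BeginPlay it hands the PlaceableImage widget to the NextPObject and LastPObject button widgets as their Texture.
; Select, deselect and teleport-click events resolve the given component to its user widget via FindComponent and forward to whichever button matches.
; Every tick the actor yaws to face the player pawn.
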(event `/Game/VRFireField/Blueprint/BaseObject/MotionInterface.BeginSelect`
  (params (SelectedComponent :type "PrimitiveComponent Object Reference"))
  ;[1 1 1] 事件调用
  (bind _widget (`self.FindComponent` SelectedComponent)
    (:`Out`
      (bind _asnext_pobject (cast `/Game/VRFireField/Blueprint/BaseObject/NextPObject` _widget)
        (:`then`
          (`/Game/VRFireField/Blueprint/BaseObject/NextPObject.BeginSelect` _asnext_pobject))
        (:`CastFailed`
          (bind _aslast_pobject (cast `/Game/VRFireField/Blueprint/BaseObject/LastPObject` _widget))
          (`/Game/VRFireField/Blueprint/BaseObject/LastPObject.BeginSelect` _aslast_pobject))))))

(event `self.ReceiveBeginPlay`
  (bind _asplaceable_image (cast `/Game/VRFireField/Blueprint/BaseObject/PlaceableImage` (`WidgetComponent.GetUserWidgetObject` (`self.Widget`)) :!pure true))
  (`|ExecutionSequence`
    (:`then_0`
      (bind _widget (`self.FindComponent` (`self.Widget2`))
        (:`Out`
          (bind _asnext_pobject (cast `/Game/VRFireField/Blueprint/BaseObject/NextPObject` _widget))
          (set `/Game/VRFireField/Blueprint/BaseObject/NextPObject.Texture` _asplaceable_image _asnext_pobject))))
    (:`then_1`
      (bind _widget_2 (`self.FindComponent` (`self.Widget1`))
        (:`Out`
          (bind _aslast_pobject (cast `/Game/VRFireField/Blueprint/BaseObject/LastPObject` _widget_2))
          (set `/Game/VRFireField/Blueprint/BaseObject/LastPObject.Texture` _asplaceable_image _aslast_pobject))))))

(event `/Game/VRFireField/Blueprint/BaseObject/MotionInterface.BeginTeleClick`
  (params (ClickTargetComponent :type "PrimitiveComponent Object Reference"))
  ;[1 1 1] 事件调用
  (bind _widget (`self.FindComponent` ClickTargetComponent)
    (:`Out`
      (bind _asnext_pobject (cast `/Game/VRFireField/Blueprint/BaseObject/NextPObject` _widget)
        (:`then`
          (`/Game/VRFireField/Blueprint/BaseObject/NextPObject.BeginClick` _asnext_pobject))
        (:`CastFailed`
          (bind _aslast_pobject (cast `/Game/VRFireField/Blueprint/BaseObject/LastPObject` _widget))
          (`/Game/VRFireField/Blueprint/BaseObject/LastPObject.BeginClick` _aslast_pobject))))))

(event `/Game/VRFireField/Blueprint/BaseObject/MotionInterface.EndSelect`
  (params (LastSelectedComponent :type "PrimitiveComponent Object Reference"))
  ;[1 1 1] 事件调用
  (bind _widget (`self.FindComponent` LastSelectedComponent)
    (:`Out`
      (bind _asnext_pobject (cast `/Game/VRFireField/Blueprint/BaseObject/NextPObject` _widget)
        (:`then`
          (`/Game/VRFireField/Blueprint/BaseObject/NextPObject.EndSelect` _asnext_pobject))
        (:`CastFailed`
          (bind _aslast_pobject (cast `/Game/VRFireField/Blueprint/BaseObject/LastPObject` _widget))
          (`/Game/VRFireField/Blueprint/BaseObject/LastPObject.EndSelect` _aslast_pobject))))))

(event `self.ReceiveTick`
  (params (DeltaSeconds :type "Float (single-precision)"))
  (bind (_returnvalue_roll _returnvalue_pitch _returnvalue_yaw) (`KismetMathLibrary.BreakRotator` (`KismetMathLibrary.FindLookAtRotation` (`self.K2_GetActorLocation`) (`self.K2_GetActorLocation` (`GameplayStatics.GetPlayerPawn` 0)))))
  (`self.K2_SetActorRotation` (`KismetMathLibrary.MakeRotator` 0.0 0.0 _returnvalue_yaw)))

(fn `UserConstructionScript`)