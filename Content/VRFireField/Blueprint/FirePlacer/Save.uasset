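; VR save panel actor in the fire placer, holding a StartSave widget and a SaveEditText widget on two widget components.
; On BeginPlay it hands the text box from SaveEditText to StartSave.
; Select, end-select and tele-click events are forwarded to whichever widget matches the targeted component.
; Each tick it turns only its yaw to face the player pawn.
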(event `self.ReceiveBeginPlay`
  (bind _asstart_save (cast `/Game/VRFireField/Blueprint/BaseObject/StartSave` (`WidgetComponent.GetUserWidgetObject` (`self.Widget`))))
  (bind _assave_edit_text (cast `/Game/VRFireField/Blueprint/BaseObject/SaveEditText` (`WidgetComponent.GetUserWidgetObject` (`self.Widget1`))))
  (set `/Game/VRFireField/Blueprint/BaseObject/StartSave.Textbox` (`/Game/VRFireField/Blueprint/BaseObject/SaveEditText.EditableTextBox_138` _assave_edit_text) _asstart_save))

(event `/Game/VRFireField/Blueprint/BaseObject/MotionInterface.BeginSelect`
  (params (SelectedComponent :type "PrimitiveComponent Object Reference"))
  (bind _aswidget_component (cast `WidgetComponent` SelectedComponent))
  (if (== _aswidget_component (`self.Widget`))
    (bind _returnvalue (`WidgetComponent.GetUserWidgetObject` _aswidget_component))
    (bind _asstart_save (cast `/Game/VRFireField/Blueprint/BaseObject/StartSave` _returnvalue))
    (`/Game/VRFireField/Blueprint/BaseObject/StartSave.BeginSelect` _asstart_save)
    (else
      (bind _assave_edit_text (cast `/Game/VRFireField/Blueprint/BaseObject/SaveEditText` _returnvalue))
      (`/Game/VRFireField/Blueprint/BaseObject/SaveEditText.BeginSelect` _assave_edit_text))))

(event `self.ReceiveTick`
  (params (DeltaSeconds :type "Float (single-precision)"))
  (bind (_returnvalue_roll _returnvalue_pitch _returnvalue_yaw) (`KismetMathLibrary.BreakRotator` (`KismetMathLibrary.FindLookAtRotation` (`self.K2_GetActorLocation`) (`self.K2_GetActorLocation` (`GameplayStatics.GetPlayerPawn` 0)))))
  (`self.K2_SetActorRotation` (`KismetMathLibrary.MakeRotator` 0.0 0.0 _returnvalue_yaw)))

(event `/Game/VRFireField/Blueprint/BaseObject/MotionInterface.BeginTeleClick`
  (params (ClickTargetComponent :type "PrimitiveComponent Object Reference"))
  (bind _aswidget_component (cast `WidgetComponent` ClickTargetComponent))
  (if (== _aswidget_component (`self.Widget`))
    (bind _returnvalue (`WidgetComponent.GetUserWidgetObject` _aswidget_component))
    (bind _asstart_save (cast `/Game/VRFireField/Blueprint/BaseObject/StartSave` _returnvalue))
    (`/Game/VRFireField/Blueprint/BaseObject/StartSave.BeginClick` _asstart_save)
    (else
      (bind _assave_edit_text (cast `/Game/VRFireField/Blueprint/BaseObject/SaveEditText` _returnvalue))
      (`/Game/VRFireField/Blueprint/BaseObject/SaveEditText.BeginClick` _assave_edit_text))))

(event `/Game/VRFireField/Blueprint/BaseObject/MotionInterface.EndSelect`
  (params (LastSelectedComponent :type "PrimitiveComponent Object Reference"))
  (bind _aswidget_component (cast `WidgetComponent` LastSelectedComponent))
  (if (== _aswidget_component (`self.Widget`))
    (bind _returnvalue (`WidgetComponent.GetUserWidgetObject` _aswidget_component))
    (bind _asstart_save (cast `/Game/VRFireField/Blueprint/BaseObject/StartSave` _returnvalue))
    (`/Game/VRFireField/Blueprint/BaseObject/StartSave.EndSelect` _asstart_save)
    (else
      (bind _assave_edit_text (cast `/Game/VRFireField/Blueprint/BaseObject/SaveEditText` _returnvalue))
      (`/Game/VRFireField/Blueprint/BaseObject/SaveEditText.EndSelect` _assave_edit_text))))

(fn `UserConstructionScript`)