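; Self-spreading fire actor with particles and audio that can be put out by damage.
; While active, it repeatedly waits a delay, then spawns a copy of itself at an unburned FireSetableVolume overlapping its attach volume and marks that volume fired.
; Damage stops spreading and destroys it after one second unless ReFire intervenes.
; It can also spawn smoke once where an upward trace hits, shortly after starting.
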(event `self.ReceiveAnyDamage`
  (params (Damage :type "Float (single-precision)") (DamageType :type "DamageType Object Reference") (InstigatedBy :type "Controller Object Reference") (DamageCauser :type "Actor Object Reference"))
  (`/Engine/EditorBlueprintResources/StandardMacros.DoOnce` false :!label _label
    (:`Completed`
      (`ActorComponent.Deactivate` (`self.ParticleSystem`))
      (set `self.Spawn` false)
      (set `self.Deactiveing` true)
      (`self.OnReadyToDistory`)
      (`KismetSystemLibrary.Delay` 1.0)
      (if (`self.Deactiveing`)
        (`self.OnDestoryed`)
        (`self.K2_DestroyActor`)
        (else
          (goto _label :!via `Reset`))))))

(event `Active`
  (bind _attachvolume (`self.AttachVolume`))
  (bind _delaytime (`self.DelayTime`))
  (`ActorComponent.SetActive` (`self.Audio`) true true)
  (`ActorComponent.SetActive` (`self.ParticleSystem`) true true)
  (set `self.Spawn` true)
  (`KismetSystemLibrary.Delay` _delaytime :!label _label_2)
  (if (and (`self.Spawn`) (!= _attachvolume null)) :!label _label_3
    (for _array_element (`self.GetOverlappingActors` _attachvolume "/Game/VRFireField/Blueprint/FireSetableVolume.FireSetableVolume_C")
      (bind _asfire_setable_volume (cast `/Game/VRFireField/Blueprint/FireSetableVolume` _array_element))
      (if (not (`/Game/VRFireField/Blueprint/FireSetableVolume.Fired` _asfire_setable_volume))
        (`|ExecutionSequence`
          (:`then_0`
            (bind _returnvalue (`|SpawnActorFromClass` (`GameplayStatics.GetObjectClass` self) (`KismetMathLibrary.MakeTransform` (`self.K2_GetActorLocation` _asfire_setable_volume)) "Undefined" "OverrideRootScale" null (select `bool` (`/Game/VRFireField/Blueprint/FireSetableVolume.CustomNextFire` _asfire_setable_volume) :`false` _delaytime :`true` (`/Game/VRFireField/Blueprint/FireSetableVolume.NextFireTime` _asfire_setable_volume)) true _asfire_setable_volume))
            (set `/Game/VRFireField/Blueprint/FireSetableVolume.Fired` true _asfire_setable_volume)
            (`/Game/VRFireField/Blueprint/FireSetableVolume.AfterFired` _asfire_setable_volume)
            (`self.OnFireSpawned` self _returnvalue))
          (:`then_1`
            (break)))))
    (goto _label_2)))

(event `DeActive`
  (`ActorComponent.Deactivate` (`self.Audio`))
  (`ActorComponent.Deactivate` (`self.ParticleSystem`))
  (set `self.Spawn` false))

(event `/Game/VRFireField/Blueprint/BaseObject/WaterableInterface.EventWeatered`
  (`self.OnWatered`))

(event `FireNext`
  (goto _label_3))

(event `self.ReceiveBeginPlay`
  (if (`self.StartActive`)
    (`self.Active`)
    (if (and (`self.CanSpawnSmoke`) (!= (`self.SmokeClass`) null))
      (`KismetSystemLibrary.K2_SetTimer` null "SpawnSmoke" 1.0)
      (goto _label_2)
      (else
        (goto _label_2)))
    (else
      (`self.DeActive`))))

(event `ReFire`
  (set `self.Spawn` true)
  (`ActorComponent.Activate` (`self.ParticleSystem`) false)
  (set `self.Deactiveing` false))

(fn `SpawnSmoke`
  (params (SmokeClass :type "Actor Class Reference"))
  (bind _returnvalue (`self.K2_GetActorLocation`))
  (bind (_outhit _returnvalue_2) (`KismetSystemLibrary.LineTraceSingle` _returnvalue (+ _returnvalue (* (`self.GetActorUpVector`) 200)) "TraceTypeQuery1"))
  (if _returnvalue_2
    (`|SpawnActorFromClass` SmokeClass (`KismetMathLibrary.MakeTransform` (`.Location` (`GameplayStatics.BreakHitResult` _outhit))) "Undefined" "OverrideRootScale")))

(fn `UserConstructionScript`)