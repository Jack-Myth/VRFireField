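; Phone is a grabbable prop in the VR fire game that the player picks up to summon firefighters.
; It records its starting transform on BeginPlay.
; On BeginCatch, unless CustomResponed is set, it detaches and snaps back to that transform, so it is never carried away.
; It then spawns temporary player-following FloatingText announcing that firefighters are coming and clears NeedToFindPhone on the FireFighter pawn.
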(event `self.ReceiveBeginPlay`
  (`parent.ReceiveBeginPlay`)
  (set `self.Transform` (`self.GetTransform`)))

(event `/Game/VRFireField/Blueprint/BaseObject/CatchableMesh.BeginCatch`
  (params (HoldingHand :type "PrimitiveComponent Object Reference"))
  (bind _returnvalue (`GameplayStatics.GetPlayerPawn` 0))
  (`parent.BeginCatch` HoldingHand)
  (if (not (`self.CustomResponed`))
    (`self.K2_DetachFromActor` "KeepRelative")
    (`self.K2_SetActorTransform` (`self.Transform`))
    (`|SpawnActorFromClass` "/Game/VRFireField/Blueprint/SenceObject/FloatingText.FloatingText_C" (`KismetMathLibrary.MakeTransform` (+ (+ (`self.K2_GetActorLocation` _returnvalue) (0.0 0.0 100.0)) (* (`self.GetActorForwardVector` _returnvalue) 100))) "Undefined" "OverrideRootScale" null "消防员正在赶来的路上" 10.0 true)
    (bind _asfire_fighter (cast `/Game/VRFireField/Blueprint/FireFighter` (`GameplayStatics.GetPlayerPawn` 0)))
    (set `/Game/VRFireField/Blueprint/FireFighter.NeedToFindPhone` false _asfire_fighter)))

(fn `UserConstructionScript`
  (`parent.UserConstructionScript`))