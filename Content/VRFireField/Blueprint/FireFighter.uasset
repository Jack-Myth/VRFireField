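; VR firefighter player pawn with stick movement, two-handed grab and use of CatchableMesh items, and hold-to-exit or reload.
; Each hand grabs from sphere overlaps, forwarding catch/use events to the held item.
; Tick moves the actor with the headset, counter-offsetting VROffset so the body follows room-scale walking.
; It also yaws a guide Cube toward the nearest Phone (if needed), MHQ extinguisher, then Fire, spawning success text when none remain.
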(event Custom|ReleaseCatch
  (params (Hand%20To%20Release :type Primitive%20Component%20Object%20Reference))
  (bind _motioncontroller_l (Variables|Default|GetMotionController_L))
  (bind _motioncontroller_r (Variables|Default|GetMotionController_R))
  (if (and (== Hand%20To%20Release (Variables|Default|GetMotionController_L)) (!= (Variables|Default|GetCatchingActorL) 0))
    ;[1 1 1] CatchActionForL
    (if (== (Variables|Default|GetCatchingActorL) 0)
      (bind _array_element (Utilities|ForEachLoopwithBreakOutput (Class|PrimitiveComponent|GetOverlappingComponents (Variables|Default|GetSphere)) :!label _label)
        (:LoopBody
          (bind _ascatchable_mesh (Utilities|Casting|CastToCatchableMesh (Components|GetOwner _array_element)))
          (if (and (and (stale _bsuccess) (.bSuccess (Utilities|Casting|CastToSphereComponent _array_element))) (not (Variables|/Game/VRFireField/Blueprint/BaseObject/CatchableMesh.CatchableMesh_C|GetCatching _ascatchable_mesh)))
            (if (Variables|/Game/VRFireField/Blueprint/BaseObject/CatchableMesh.CatchableMesh_C|GetHoldable _ascatchable_mesh)
              (Physics|SetSimulatePhysics (Variables|/Script/Engine.StaticMeshActor|GetStaticMeshComponent _ascatchable_mesh) false)
              (Transformation|AttachComponentToComponent _ascatchable_mesh _motioncontroller_l "None" "SnapToTarget" "SnapToTarget" "KeepWorld" true)
              (Transformation|SetActorRelativeTransform _ascatchable_mesh (Math|Transform|MakeTransform (Math|Vector|MakeVector (* (.x (* (.location (Variables|/Game/VRFireField/Blueprint/BaseObject/CatchableMesh.CatchableMesh_C|GetTransformOffsetL _ascatchable_mesh)) -1)) (.X (Math|Vector|BreakVector (Transformation|GetActorScale3D _ascatchable_mesh)))) (* (.y (* (.location (Variables|/Game/VRFireField/Blueprint/BaseObject/CatchableMesh.CatchableMesh_C|GetTransformOffsetL _ascatchable_mesh)) -1)) (.Y (Math|Vector|BreakVector (Transformation|GetActorScale3D _ascatchable_mesh)))) (* (.z (* (.location (Variables|/Game/VRFireField/Blueprint/BaseObject/CatchableMesh.CatchableMesh_C|GetTransformOffsetL _ascatchable_mesh)) -1)) (.Z (Math|Vector|BreakVector (Transformation|GetActorScale3D _ascatchable_mesh))))) (.rotation (Variables|/Game/VRFireField/Blueprint/BaseObject/CatchableMesh.CatchableMesh_C|GetTransformOffsetL _ascatchable_mesh)) (Transformation|GetActorScale3D _ascatchable_mesh)) false false))
            (bind _output_get (Variables|Default|SetCatchingActorL _ascatchable_mesh))
            (Collision|SetCollisionEnabled (Variables|/Script/Engine.StaticMeshActor|GetStaticMeshComponent _ascatchable_mesh) "QueryOnly")
            (Components|Animation|PlayAnimation (Variables|Default|GetSkeletalMesh1) "/Game/VirtualReality/Mannequin/Animations/MannequinHand_Right_Grab.MannequinHand_Right_Grab" false)
            (Default|BeginCatch _output_get (Variables|Default|GetMotionController_L))
            (goto _label Break))))
      (else
        (Transformation|DetachFromActor (Variables|Default|GetCatchingActorL) "KeepWorld" "KeepWorld" "KeepWorld")
        (Collision|SetCollisionEnabled (Variables|/Script/Engine.StaticMeshActor|GetStaticMeshComponent (Variables|Default|GetCatchingActorL)) "QueryAndPhysics")
        (if (Variables|/Game/VRFireField/Blueprint/BaseObject/CatchableMesh.CatchableMesh_C|GetHoldable (Variables|Default|GetCatchingActorL))
          (Physics|SetSimulatePhysics (Variables|/Script/Engine.StaticMeshActor|GetStaticMeshComponent (Variables|Default|GetCatchingActorL)) true))
        (Default|EndCatch (Variables|Default|GetCatchingActorL) _motioncontroller_l)
        (Components|Animation|PlayAnimation (Variables|Default|GetSkeletalMesh1) "/Game/VirtualReality/Mannequin/Animations/MannequinHand_Right_Open.MannequinHand_Right_Open" false)
        (if (Variables|Default|GetUsingL)
          (Default|EndUse (Variables|Default|GetCatchingActorL) _motioncontroller_l))
        (Variables|Default|SetCatchingActorL 0)))
    (elif (and (== Hand%20To%20Release (Variables|Default|GetMotionController_R)) (!= (Variables|Default|GetCatchingActorR) 0))
      ;[1 1 1] CatchActionForR
      (if (== (Variables|Default|GetCatchingActorR) 0)
        (bind _array_element_2 (Utilities|ForEachLoopwithBreakOutput (Class|PrimitiveComponent|GetOverlappingComponents (Variables|Default|GetSphereR)) :!label _label_2)
          (:LoopBody
            (bind _ascatchable_mesh_2 (Utilities|Casting|CastToCatchableMesh (Components|GetOwner _array_element_2)))
            (if (and (and (stale _bsuccess) (.bSuccess (Utilities|Casting|CastToSphereComponent _array_element_2))) (not (Variables|/Game/VRFireField/Blueprint/BaseObject/CatchableMesh.CatchableMesh_C|GetCatching _ascatchable_mesh_2)))
              (if (Variables|/Game/VRFireField/Blueprint/BaseObject/CatchableMesh.CatchableMesh_C|GetHoldable _ascatchable_mesh_2)
                (Physics|SetSimulatePhysics (Variables|/Script/Engine.StaticMeshActor|GetStaticMeshComponent _ascatchable_mesh_2) false)
                (Transformation|AttachComponentToComponent _ascatchable_mesh_2 _motioncontroller_r "None" "SnapToTarget" "SnapToTarget" "KeepWorld" true)
                (Transformation|SetActorRelativeTransform _ascatchable_mesh_2 (Math|Transform|MakeTransform (Math|Vector|MakeVector (* (.x (* (.location (Variables|/Game/VRFireField/Blueprint/BaseObject/CatchableMesh.CatchableMesh_C|GetTransformOffsetR _ascatchable_mesh_2)) -1)) (.X (Math|Vector|BreakVector (Transformation|GetActorScale3D _ascatchable_mesh_2)))) (* (.y (* (.location (Variables|/Game/VRFireField/Blueprint/BaseObject/CatchableMesh.CatchableMesh_C|GetTransformOffsetR _ascatchable_mesh_2)) -1)) (.Y (Math|Vector|BreakVector (Transformation|GetActorScale3D _ascatchable_mesh_2)))) (* (.z (* (.location (Variables|/Game/VRFireField/Blueprint/BaseObject/CatchableMesh.CatchableMesh_C|GetTransformOffsetR _ascatchable_mesh_2)) -1)) (.Z (Math|Vector|BreakVector (Transformation|GetActorScale3D _ascatchable_mesh_2))))) (.rotation (Variables|/Game/VRFireField/Blueprint/BaseObject/CatchableMesh.CatchableMesh_C|GetTransformOffsetR _ascatchable_mesh_2)) (Transformation|GetActorScale3D _ascatchable_mesh_2)) false false))
              (bind _output_get_2 (Variables|Default|SetCatchingActorR _ascatchable_mesh_2))
              (Collision|SetCollisionEnabled (Variables|/Script/Engine.StaticMeshActor|GetStaticMeshComponent _ascatchable_mesh_2) "QueryOnly")
              (Components|Animation|PlayAnimation (Variables|Default|GetSkeletalMesh) "/Game/VirtualReality/Mannequin/Animations/MannequinHand_Right_Grab.MannequinHand_Right_Grab" false)
              (Default|BeginCatch _output_get_2 (Variables|Default|GetMotionController_R))
              (goto _label_2 Break))))
        (else
          (Transformation|DetachFromActor (Variables|Default|GetCatchingActorR) "KeepWorld" "KeepWorld" "KeepWorld")
          (Collision|SetCollisionEnabled (Variables|/Script/Engine.StaticMeshActor|GetStaticMeshComponent (Variables|Default|GetCatchingActorR)) "QueryAndPhysics")
          (if (Variables|/Game/VRFireField/Blueprint/BaseObject/CatchableMesh.CatchableMesh_C|GetHoldable (Variables|Default|GetCatchingActorR))
            (Physics|SetSimulatePhysics (Variables|/Script/Engine.StaticMeshActor|GetStaticMeshComponent (Variables|Default|GetCatchingActorR)) true))
          (Default|EndCatch (Variables|Default|GetCatchingActorR) _motioncontroller_r)
          (Components|Animation|PlayAnimation (Variables|Default|GetSkeletalMesh) "/Game/VirtualReality/Mannequin/Animations/MannequinHand_Right_Open.MannequinHand_Right_Open" false)
          (if (Variables|Default|GetUsingR)
            (Default|EndUse (Variables|Default|GetCatchingActorR) _motioncontroller_r))
          (Variables|Default|SetCatchingActorR 0))))))

(event EventBeginPlay
  (Class|HeadMountedDisplayFunctionLibrary|EnableHMD true)
  (if (Class|HeadMountedDisplayFunctionLibrary|IsHeadMountedDisplayEnabled)
    (Utilities|Time|SetTimerbyFunctionName 0 "CheckA" 1.0 true)))

(event EventTick
  (params (DeltaSeconds :type Float%20%28single-precision%29))
  (bind _deviceposition (Class|HeadMountedDisplayFunctionLibrary|GetOrientationandPosition))
  (bind _returnvalue (Transformation|GetActorLocation))
  (bind _deviceposition_2 (Class|HeadMountedDisplayFunctionLibrary|GetOrientationandPosition))
  (bind _returnvalue_2 (Game|Player|GetPlayerPawn 0))
  (bind _vroffset (Variables|Default|GetVROffset))
  ;[1 1 1] TickForGuide
  (if (Class|HeadMountedDisplayFunctionLibrary|IsHeadMountedDisplayEnabled)
    (Transformation|SetActorLocation (Math|Vector|MakeVector (+ (.x _returnvalue) (.x (- _deviceposition_2 (Variables|Default|GetPersonLastPosition)))) (+ (.y _returnvalue) (.y (- _deviceposition_2 (Variables|Default|GetPersonLastPosition)))) (.z _returnvalue)) true false)
    (Transformation|SetRelativeLocation _vroffset (Math|Vector|MakeVector (* -1 (.x _deviceposition)) (* -1 (.y _deviceposition)) (.z (Variables|/Script/Engine.SceneComponent|GetRelativeLocation _vroffset))) false false)
    (Variables|Default|SetPersonLastPosition _deviceposition_2))
  (if (Variables|Default|GetNeedToFindPhone)
    (bind _outactors (Actor|GetAllActorsOfClass "/Game/VRFireField/Blueprint/Phone.Phone_C"))
    (if (== (Utilities|Array|Length _outactors) 0)
      (if (or (.bSuccess (Utilities|Casting|CastToMHQ (Variables|Default|GetCatchingActorR))) (.bSuccess (Utilities|Casting|CastToMHQ (Variables|Default|GetCatchingActorL)))) :!label _label
        (bind _outactors_2 (Actor|GetAllActorsOfClass "/Game/VRFireField/Blueprint/Fire.Fire_C"))
        (if (!= (Utilities|Array|Length _outactors_2) 0)
          (bind _mostcloseactorindex (CallFunction|GetMostCloseActor _outactors_2))
          (Transformation|SetWorldRotation (Variables|Default|GetCube) (Math|Rotator|MakeRotator 0.0 0.0 (+ (.yaw (Math|Rotator|FindLookatRotation (Transformation|GetActorLocation (Game|Player|GetPlayerPawn 0)) (Transformation|GetActorLocation (Utilities|Array|Get(acopy) _outactors_2 _mostcloseactorindex)))) 9e+01)) false false)
          (else
            (Actor|Tick|SetActorTickEnabled false)
            (Rendering|SetVisibility (Variables|Default|GetCube) false false)
            (Game|SpawnActorfromClass "/Game/VRFireField/Blueprint/SenceObject/FloatingText.FloatingText_C" (Math|Transform|MakeTransform (+ (+ (Transformation|GetActorLocation _returnvalue_2) "0, 0,50.000000") (* (Transformation|GetActorForwardVector _returnvalue_2) 100)) "0, 0, 0" "1,1.000000,1") "Undefined" 0 "灭火成功" 0.0 true)))
        (else
          (bind _outactors_3 (Actor|GetAllActorsOfClass "/Game/VRFireField/Blueprint/MHQ.MHQ_C"))
          (bind _mostcloseactorindex_2 (CallFunction|GetMostCloseActor _outactors_3))
          (Transformation|SetWorldRotation (Variables|Default|GetCube) (Math|Rotator|MakeRotator 0.0 0.0 (+ (.yaw (Math|Rotator|FindLookatRotation (Transformation|GetActorLocation (Game|Player|GetPlayerPawn 0)) (Transformation|GetActorLocation (Utilities|Array|Get(acopy) _outactors_3 _mostcloseactorindex_2)))) 9e+01)) false false)))
      (else
        (bind _mostcloseactorindex_3 (CallFunction|GetMostCloseActor _outactors))
        (Transformation|SetWorldRotation (Variables|Default|GetCube) (Math|Rotator|MakeRotator 0.0 0.0 (+ (.yaw (Math|Rotator|FindLookatRotation (Transformation|GetActorLocation (Game|Player|GetPlayerPawn 0)) (Transformation|GetActorLocation (Utilities|Array|Get(acopy) _outactors _mostcloseactorindex_3)))) 9e+01)) false false)))
    (else
      (goto _label))))

(event Input|ActionEvents|InputActionExit
  (params (Key :type Key%20Structure :default "AnyKey"))
  ;[1 1 1] Exit
  (:Pressed
    (Utilities|ForLoopwithDelay 1 100 0.02 :!label _label
      (:Complited
        (bind _returnvalue (Game|GetCurrentLevelName true))
        (if (Utilities|Enum|Equal(Enum) _returnvalue "Main_Menu")
          (Game|QuitGame 0 "Quit")
          (else
            (Game|OpenLevel(byName) "Main_Menu"))))))
  (:Released
    (goto _label Break)))

(event Input|ActionEvents|InputActionReLoadMap
  (params (Key :type Key%20Structure :default "AnyKey"))
  ;[1 1 1] Exit
  (:Pressed
    (Utilities|ForLoopwithDelay 1 100 0.02 :!label _label
      (:Complited
        (bind _returnvalue (Game|GetCurrentLevelName true))
        (Game|OpenLevel(byName) (Utilities|String|StringToName _returnvalue)))))
  (:Released
    (goto _label Break)))

(event Input|ActionEvents|InputActionActionForL
  (params (Key :type Key%20Structure :default "AnyKey"))
  (bind _motioncontroller_l (Variables|Default|GetMotionController_L))
  (bind _catchingactorl (Variables|Default|GetCatchingActorL))
  (bind _returnvalue (!= _catchingactorl 0))
  ;[1 1 1] ActionForRelease
  (:Pressed
    (if _returnvalue
      (Variables|Default|SetUsingL true)
      (Default|BeginUse _catchingactorl _motioncontroller_l)))
  (:Released
    (if _returnvalue
      (Variables|Default|SetUsingL false)
      (Default|EndUse _catchingactorl _motioncontroller_l))))

(event Input|ActionEvents|InputActionActionForR
  (params (Key :type Key%20Structure :default "AnyKey"))
  (bind _catchingactorr (Variables|Default|GetCatchingActorR))
  (bind _motioncontroller_r (Variables|Default|GetMotionController_R))
  (bind _returnvalue (!= _catchingactorr 0))
  ;[1 1 1] ActionForRelease
  (:Pressed
    (if _returnvalue
      (Variables|Default|SetUsingR true)
      (Default|BeginUse _catchingactorr _motioncontroller_r)))
  (:Released
    (if _returnvalue
      (Variables|Default|SetUsingR false)
      (Default|EndUse _catchingactorr _motioncontroller_r))))

(event Input|ActionEvents|InputActionAllowMove
  (params (Key :type Key%20Structure :default "AnyKey"))
  ;[1 1 1] Movement
  (:Pressed
    (Variables|Default|SetAllowMove true))
  (:Released
    (Variables|Default|SetAllowMove false)))

(event Input|ActionEvents|InputActionCatchActionForR
  (params (Key :type Key%20Structure :default "AnyKey"))
  (bind _motioncontroller_r (Variables|Default|GetMotionController_R))
  ;[1 1 1] CatchActionForR
  (:Pressed
    (if (== (Variables|Default|GetCatchingActorR) 0)
      (bind _array_element (Utilities|ForEachLoopwithBreakOutput (Class|PrimitiveComponent|GetOverlappingComponents (Variables|Default|GetSphereR)) :!label _label)
        (:LoopBody
          (bind _ascatchable_mesh (Utilities|Casting|CastToCatchableMesh (Components|GetOwner _array_element)))
          (if (and (and (stale _bsuccess) (.bSuccess (Utilities|Casting|CastToSphereComponent _array_element))) (not (Variables|/Game/VRFireField/Blueprint/BaseObject/CatchableMesh.CatchableMesh_C|GetCatching _ascatchable_mesh)))
            (if (Variables|/Game/VRFireField/Blueprint/BaseObject/CatchableMesh.CatchableMesh_C|GetHoldable _ascatchable_mesh)
              (Physics|SetSimulatePhysics (Variables|/Script/Engine.StaticMeshActor|GetStaticMeshComponent _ascatchable_mesh) false)
              (Transformation|AttachComponentToComponent _ascatchable_mesh _motioncontroller_r "None" "SnapToTarget" "SnapToTarget" "KeepWorld" true)
              (Transformation|SetActorRelativeTransform _ascatchable_mesh (Math|Transform|MakeTransform (Math|Vector|MakeVector (* (.x (* (.location (Variables|/Game/VRFireField/Blueprint/BaseObject/CatchableMesh.CatchableMesh_C|GetTransformOffsetR _ascatchable_mesh)) -1)) (.X (Math|Vector|BreakVector (Transformation|GetActorScale3D _ascatchable_mesh)))) (* (.y (* (.location (Variables|/Game/VRFireField/Blueprint/BaseObject/CatchableMesh.CatchableMesh_C|GetTransformOffsetR _ascatchable_mesh)) -1)) (.Y (Math|Vector|BreakVector (Transformation|GetActorScale3D _ascatchable_mesh)))) (* (.z (* (.location (Variables|/Game/VRFireField/Blueprint/BaseObject/CatchableMesh.CatchableMesh_C|GetTransformOffsetR _ascatchable_mesh)) -1)) (.Z (Math|Vector|BreakVector (Transformation|GetActorScale3D _ascatchable_mesh))))) (.rotation (Variables|/Game/VRFireField/Blueprint/BaseObject/CatchableMesh.CatchableMesh_C|GetTransformOffsetR _ascatchable_mesh)) (Transformation|GetActorScale3D _ascatchable_mesh)) false false))
            (bind _output_get (Variables|Default|SetCatchingActorR _ascatchable_mesh))
            (Collision|SetCollisionEnabled (Variables|/Script/Engine.StaticMeshActor|GetStaticMeshComponent _ascatchable_mesh) "QueryOnly")
            (Components|Animation|PlayAnimation (Variables|Default|GetSkeletalMesh) "/Game/VirtualReality/Mannequin/Animations/MannequinHand_Right_Grab.MannequinHand_Right_Grab" false)
            (Default|BeginCatch _output_get (Variables|Default|GetMotionController_R))
            (goto _label Break))))
      (else
        (Transformation|DetachFromActor (Variables|Default|GetCatchingActorR) "KeepWorld" "KeepWorld" "KeepWorld")
        (Collision|SetCollisionEnabled (Variables|/Script/Engine.StaticMeshActor|GetStaticMeshComponent (Variables|Default|GetCatchingActorR)) "QueryAndPhysics")
        (if (Variables|/Game/VRFireField/Blueprint/BaseObject/CatchableMesh.CatchableMesh_C|GetHoldable (Variables|Default|GetCatchingActorR))
          (Physics|SetSimulatePhysics (Variables|/Script/Engine.StaticMeshActor|GetStaticMeshComponent (Variables|Default|GetCatchingActorR)) true))
        (Default|EndCatch (Variables|Default|GetCatchingActorR) _motioncontroller_r)
        (Components|Animation|PlayAnimation (Variables|Default|GetSkeletalMesh) "/Game/VirtualReality/Mannequin/Animations/MannequinHand_Right_Open.MannequinHand_Right_Open" false)
        (if (Variables|Default|GetUsingR)
          (Default|EndUse (Variables|Default|GetCatchingActorR) _motioncontroller_r))
        (Variables|Default|SetCatchingActorR 0)))))

(event Input|ActionEvents|InputActionCatchActionForL
  (params (Key :type Key%20Structure :default "AnyKey"))
  (bind _motioncontroller_l (Variables|Default|GetMotionController_L))
  ;[1 1 1] CatchActionForL
  (:Pressed
    (if (== (Variables|Default|GetCatchingActorL) 0)
      (bind _array_element (Utilities|ForEachLoopwithBreakOutput (Class|PrimitiveComponent|GetOverlappingComponents (Variables|Default|GetSphere)) :!label _label)
        (:LoopBody
          (bind _ascatchable_mesh (Utilities|Casting|CastToCatchableMesh (Components|GetOwner _array_element)))
          (if (and (and (stale _bsuccess) (.bSuccess (Utilities|Casting|CastToSphereComponent _array_element))) (not (Variables|/Game/VRFireField/Blueprint/BaseObject/CatchableMesh.CatchableMesh_C|GetCatching _ascatchable_mesh)))
            (if (Variables|/Game/VRFireField/Blueprint/BaseObject/CatchableMesh.CatchableMesh_C|GetHoldable _ascatchable_mesh)
              (Physics|SetSimulatePhysics (Variables|/Script/Engine.StaticMeshActor|GetStaticMeshComponent _ascatchable_mesh) false)
              (Transformation|AttachComponentToComponent _ascatchable_mesh _motioncontroller_l "None" "SnapToTarget" "SnapToTarget" "KeepWorld" true)
              (Transformation|SetActorRelativeTransform _ascatchable_mesh (Math|Transform|MakeTransform (Math|Vector|MakeVector (* (.x (* (.location (Variables|/Game/VRFireField/Blueprint/BaseObject/CatchableMesh.CatchableMesh_C|GetTransformOffsetL _ascatchable_mesh)) -1)) (.X (Math|Vector|BreakVector (Transformation|GetActorScale3D _ascatchable_mesh)))) (* (.y (* (.location (Variables|/Game/VRFireField/Blueprint/BaseObject/CatchableMesh.CatchableMesh_C|GetTransformOffsetL _ascatchable_mesh)) -1)) (.Y (Math|Vector|BreakVector (Transformation|GetActorScale3D _ascatchable_mesh)))) (* (.z (* (.location (Variables|/Game/VRFireField/Blueprint/BaseObject/CatchableMesh.CatchableMesh_C|GetTransformOffsetL _ascatchable_mesh)) -1)) (.Z (Math|Vector|BreakVector (Transformation|GetActorScale3D _ascatchable_mesh))))) (.rotation (Variables|/Game/VRFireField/Blueprint/BaseObject/CatchableMesh.CatchableMesh_C|GetTransformOffsetL _ascatchable_mesh)) (Transformation|GetActorScale3D _ascatchable_mesh)) false false))
            (bind _output_get (Variables|Default|SetCatchingActorL _ascatchable_mesh))
            (Collision|SetCollisionEnabled (Variables|/Script/Engine.StaticMeshActor|GetStaticMeshComponent _ascatchable_mesh) "QueryOnly")
            (Components|Animation|PlayAnimation (Variables|Default|GetSkeletalMesh1) "/Game/VirtualReality/Mannequin/Animations/MannequinHand_Right_Grab.MannequinHand_Right_Grab" false)
            (Default|BeginCatch _output_get (Variables|Default|GetMotionController_L))
            (goto _label Break))))
      (else
        (Transformation|DetachFromActor (Variables|Default|GetCatchingActorL) "KeepWorld" "KeepWorld" "KeepWorld")
        (Collision|SetCollisionEnabled (Variables|/Script/Engine.StaticMeshActor|GetStaticMeshComponent (Variables|Default|GetCatchingActorL)) "QueryAndPhysics")
        (if (Variables|/Game/VRFireField/Blueprint/BaseObject/CatchableMesh.CatchableMesh_C|GetHoldable (Variables|Default|GetCatchingActorL))
          (Physics|SetSimulatePhysics (Variables|/Script/Engine.StaticMeshActor|GetStaticMeshComponent (Variables|Default|GetCatchingActorL)) true))
        (Default|EndCatch (Variables|Default|GetCatchingActorL) _motioncontroller_l)
        (Components|Animation|PlayAnimation (Variables|Default|GetSkeletalMesh1) "/Game/VirtualReality/Mannequin/Animations/MannequinHand_Right_Open.MannequinHand_Right_Open" false)
        (if (Variables|Default|GetUsingL)
          (Default|EndUse (Variables|Default|GetCatchingActorL) _motioncontroller_l))
        (Variables|Default|SetCatchingActorL 0)))))

(event Input|AxisEvents|InputAxisMoveForword
  (params (AxisValue :type Float%20%28single-precision%29))
  ;[1 1 1] Movement
  (if (Variables|Default|GetAllowMove)
    (Pawn|Input|AddMovementInput (Math|Vector|GetForwardVector (Math|Rotator|MakeRotator 0.0 0.0 (.yaw (Transformation|GetWorldRotation (Variables|Default|GetCamera))))) (/ AxisValue 4.0) false)))

(event Input|AxisEvents|InputAxisViewX
  (params (AxisValue :type Float%20%28single-precision%29))
  ;[1 1 1] Movement
  (Pawn|Input|AddControllerYawInput AxisValue))

(event Input|AxisEvents|InputAxisViewY
  (params (AxisValue :type Float%20%28single-precision%29))
  ;[1 1 1] Movement
  (Pawn|Input|AddControllerPitchInput AxisValue))

(event Input|AxisEvents|InputAxisMoveRight
  (params (AxisValue :type Float%20%28single-precision%29))
  ;[1 1 1] Movement
  (if (Variables|Default|GetAllowMove)
    (Pawn|Input|AddMovementInput (Math|Vector|GetRightVector (Math|Rotator|MakeRotator 0.0 0.0 (.yaw (Transformation|GetWorldRotation (Variables|Default|GetCamera))))) (/ AxisValue 4.0) false)))

(event Input|KeyboardEvents|K
  (params (Key :type Key%20Structure :default "AnyKey"))
  (:Pressed
    (Transformation|SetRelativeLocationAndRotation (Variables|Default|GetMotionController_R) "15.500000,10.400000,144.929993" "44.880001,-16.160000,-2.450000" false false)))

(fn ConstructionScript)

(fn CheckA
  (Transformation|SetActorRotation (Math|Rotator|MakeRotator 0.0 0.0 0.0)))

(fn GetMostCloseActor
  (params (Actors :type Array%20of%20Placeable%20Mesh%20Actor%20Object%20References))
  (for (_array_element _array_index) Actors
    (if (< (Math|Vector|VectorLength (- (Transformation|GetActorLocation (Game|Player|GetPlayerPawn 0)) (Transformation|GetActorLocation _array_element))) (LocalVariables|GetDestances))
      (LocalVariables|SetIndex _array_index)
      (LocalVariables|SetDestances (Math|Vector|VectorLength (- (Transformation|GetActorLocation (Game|Player|GetPlayerPawn 0)) (Transformation|GetActorLocation _array_element))))))
  (return (LocalVariables|GetIndex)))

(fn GetHandModel
  (params (Hand :type Primitive%20Component%20Object%20Reference))
  (if (== Hand (Variables|Default|GetMotionController_L))
    (return (Variables|Default|GetSkeletalMesh1))
    (elif (== Hand (Variables|Default|GetMotionController_R))
      (return (Variables|Default|GetSkeletalMesh))
      (else
        (return 0)))))