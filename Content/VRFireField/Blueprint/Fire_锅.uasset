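; Pot fire actor for a VR firefighting scene that grows when handled wrongly and goes out otherwise.
; Damage of exactly 1 shows the center actor's "wrong method, fire got bigger" warning and starts a one-second timer, which spawns another fire copy nearby and hides the warning.
; Other damage deactivates the particles, then after a delay calls ready-to-destroy and destroys the actor unless Spawn is set again.
; Tick turns the warning widget toward the player.
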(event `self.ReceiveAnyDamage`
  (params (Damage :type "Float (single-precision)") (DamageType :type "DamageType Object Reference") (InstigatedBy :type "Controller Object Reference") (DamageCauser :type "Actor Object Reference"))
  (if (== Damage 1.0)
    (if (not (`KismetSystemLibrary.K2_IsValidTimerHandle` (`self.AddFireTimerHandle`)))
      (bind _returnvalue (`KismetSystemLibrary.K2_SetTimer` null "AddFire" 1.0))
      (set `self.AddFireTimerHandle` _returnvalue)
      (`SceneComponent.SetVisibility` (`/Game/VRFireField/Blueprint/Fire_锅.Widget` (`self.CenterActor`)) true false))
    (else
      (bind _output_get (set `self.Spawn` false))
      (`ActorComponent.Deactivate` (`self.ParticleSystem`))
      (`/Engine/EditorBlueprintResources/StandardMacros.DoOnce` false :!label _label
        (:`Completed`
          (`KismetSystemLibrary.Delay` 2.0)
          (if _output_get
            (goto _label :!via `Reset`)
            (else
              (`self.OnReadyToDistory`)
              (`self.K2_DestroyActor`))))))))

(event `self.ReceiveBeginPlay`
  (bind _astext_r (cast `/Game/VRFireField/Blueprint/TextR` (`WidgetComponent.GetUserWidgetObject` (`self.Widget`)) :!pure true))
  (`/Game/VRFireField/Blueprint/TextR.SetText` _astext_r "做法不正确，火变的更大了")
  (`/Game/VRFireField/Blueprint/TextR.SetColor` _astext_r (struct :`A` 1.0)))

(event `self.ReceiveTick`
  (params (DeltaSeconds :type "Float (single-precision)"))
  (bind _widget (`self.Widget`))
  (`SceneComponent.K2_SetWorldRotation` _widget (`KismetMathLibrary.FindLookAtRotation` (`SceneComponent.K2_GetComponentLocation` _widget) (`self.K2_GetActorLocation` (`GameplayStatics.GetPlayerPawn` 0))) false false))

(fn `AddFire`
  (bind (_returnvalue_x _returnvalue_y _returnvalue_z) (`KismetMathLibrary.BreakVector` (`self.K2_GetActorLocation` (`self.CenterActor`))))
  (`|SpawnActorFromClass` "Fire_锅_C" (`KismetMathLibrary.MakeTransform` (`KismetMathLibrary.MakeVector` (+ _returnvalue_x (`KismetMathLibrary.RandomFloatInRange` -5.0 5.0)) (+ _returnvalue_y (`KismetMathLibrary.RandomFloatInRange` -5.0 5.0)) _returnvalue_z) (struct) (0.3 0.3 0.3)) "Undefined" "OverrideRootScale" null (`self.CenterActor`) 100.0 true)
  (`KismetSystemLibrary.K2_ClearAndInvalidateTimerHandle` (`self.AddFireTimerHandle`))
  (`SceneComponent.SetVisibility` (`/Game/VRFireField/Blueprint/Fire_锅.Widget` (`self.CenterActor`)) false false))

(fn `UserConstructionScript`
  (`parent.UserConstructionScript`))