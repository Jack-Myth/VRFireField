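; CatchableMesh is a VR grabbable mesh base that forwards catch, use and mesh overlap events through CallOn hooks.
; A text label billboards toward the player, appearing on label sphere overlap and hiding while held.
; Tick restores the initial transform after a fall out of the world; an optional timer samples velocity from position deltas.
; A static-mesh-actor flag disables tick and strips the catch and label components.
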(event `self.ReceiveBeginPlay`
  (if (`self.UseAsStaticMeshActor`)
    (`self.SetActorTickEnabled` false)
    (`ActorComponent.K2_DestroyComponent` (`self.Sphere_Catch`))
    (`ActorComponent.K2_DestroyComponent` (`self.Widget`))
    (`ActorComponent.K2_DestroyComponent` (`self.Sphere_Lable`))
    (else
      (`/Game/VRFireField/Blueprint/TextR.SetText` (cast `/Game/VRFireField/Blueprint/TextR` (`WidgetComponent.GetUserWidgetObject` (`self.Widget`)) :!pure true) (`self.DisplayLable`))
      (set `self.InitialTransform` (`self.GetTransform`))))
  (if (`self.InitCaculateSpeed`)
    (`KismetSystemLibrary.K2_SetTimer` null "CaculateSpeed" 0.1 true)))

(event `BeginCatch`
  (params (HoldingHand :type "PrimitiveComponent Object Reference"))
  (set `self.Catching` true)
  (`SceneComponent.SetVisibility` (`self.Widget`) false false)
  (`self.OnBeginCatch` HoldingHand))

(event `self.ReceiveTick`
  (params (DeltaSeconds :type "Float (single-precision)"))
  (bind (_returnvalue_x _returnvalue_y _returnvalue_z) (`KismetMathLibrary.BreakVector` (`self.K2_GetActorLocation`)))
  (bind _widget (`self.Widget`))
  (`SceneComponent.K2_SetWorldRotation` _widget (`KismetMathLibrary.FindLookAtRotation` (`SceneComponent.K2_GetComponentLocation` _widget) (+ (`self.K2_GetActorLocation` (`GameplayStatics.GetPlayerPawn` 0)) (0.0 0.0 150.0))) false false)
  (`SceneComponent.K2_SetWorldLocation` (`self.Widget`) (+ (`self.K2_GetActorLocation`) (0.0 0.0 54.0)) false false)
  (if (< _returnvalue_z -1000.0)
    (`PrimitiveComponent.SetSimulatePhysics` (`self.StaticMeshComponent`) false)
    (`self.K2_SetActorTransform` (`self.InitialTransform`))))

(event `EndCatch`
  (params (LastHoldHand :type "PrimitiveComponent Object Reference"))
  (set `self.Catching` false)
  (`self.OnEndCatch` LastHoldHand))

(event `BeginUse`
  (params (HoldingHand :type "PrimitiveComponent Object Reference"))
  (`self.OnBeginUse` HoldingHand))

(event `self.StaticMeshComponent.OnComponentBeginOverlap`
  (params (OverlappedComponent :type "PrimitiveComponent Object Reference") (OtherActor :type "Actor Object Reference") (OtherComp :type "PrimitiveComponent Object Reference") (OtherBodyIndex :type Integer) (bFromSweep :type Boolean) (SweepResult :type "HitResult Structure (by ref)"))
  (`self.OnStaticMeshComponentBeginOverlap` OverlappedComponent OtherActor OtherComp OtherBodyIndex bFromSweep SweepResult))

(event `self.Sphere_Lable.OnComponentBeginOverlap`
  (params (OverlappedComponent :type "PrimitiveComponent Object Reference") (OtherActor :type "Actor Object Reference") (OtherComp :type "PrimitiveComponent Object Reference") (OtherBodyIndex :type Integer) (bFromSweep :type Boolean) (SweepResult :type "HitResult Structure (by ref)"))
  (if (not (`self.Catching`))
    (`SceneComponent.SetVisibility` (`self.Widget`) true false)))

(event `EndUse`
  (params (HouldingHand :type "PrimitiveComponent Object Reference"))
  (`self.OnEndUse` HouldingHand))

(event `self.Sphere_Lable.OnComponentEndOverlap`
  (params (OverlappedComponent :type "PrimitiveComponent Object Reference") (OtherActor :type "Actor Object Reference") (OtherComp :type "PrimitiveComponent Object Reference") (OtherBodyIndex :type Integer))
  (if (not (`self.Catching`))
    (`SceneComponent.SetVisibility` (`self.Widget`) false false)))

(fn `CaculateSpeed`
  (bind _returnvalue (`self.K2_GetActorLocation`))
  (set `self.Speed` (* (- _returnvalue (`self.LastLocation`)) 10))
  (set `self.LastLocation` _returnvalue))

(fn `UserConstructionScript`)