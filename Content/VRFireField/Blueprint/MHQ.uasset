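; MHQ is a grabbable VR fire extinguisher that records an enum value in the game instance's 灭火器 variable when caught.
; Using it plays audio, attaches a steam particle jet and repeatedly line-traces forward, applying damage to the hit actor until use ends.
; From BeginPlay, a one-second polling loop reapplies the metal and red materials whenever the red body slot differs.
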(event `self.BeginUse`
  (params (HoldingHand :type "PrimitiveComponent Object Reference"))
  (bind _scene (`self.Scene`))
  (bind _returnvalue (`SceneComponent.K2_GetComponentLocation` _scene))
  (`ActorComponent.Activate` (`self.Audio`) true)
  (bind _returnvalue_2 (`GameplayStatics.SpawnEmitterAttached` "/Game/VRFireField/Particle/P_Steam_Lit.P_Steam_Lit" (`self.Scene`) "None" (-10.0 0.0 0.0) (struct)))
  (`/Game/MacroLibrary.Loop_Infinited` 0.1 :!label _label
    (:`LoopBody`
      (bind _outhit (`KismetSystemLibrary.LineTraceSingle` _returnvalue (+ _returnvalue (* (`SceneComponent.GetForwardVector` _scene) 500)) "TraceTypeQuery1"))
      (`GameplayStatics.ApplyDamage` (`.HitActor` (`GameplayStatics.BreakHitResult` _outhit)) (`self.Damage`)))))

(event `self.EndUse`
  (params (HouldingHand :type "PrimitiveComponent Object Reference"))
  (`ActorComponent.Deactivate` (`self.Audio`))
  (`ActorComponent.Deactivate` (stale `self.BeginUse` _returnvalue_2))
  (goto _label :!via `Break`))

(event `self.BeginCatch`
  (params (HoldingHand :type "PrimitiveComponent Object Reference"))
  (`parent.BeginCatch` null)
  (set `/Game/VRFireField/Blueprint/DefaultGameInstance.灭火器` "NewEnumerator0" (`/Game/VRFireField/GameMacro.GetGameInstance`)))

(event `self.ReceiveBeginPlay`
  (bind _staticmeshcomponent (`self.StaticMeshComponent`))
  (`parent.ReceiveBeginPlay`)
  (if (!= (`PrimitiveComponent.GetMaterial` _staticmeshcomponent 2) "/Game/VRFireField/Material/Color_Red.Color_Red") :!label _label_2
    (`PrimitiveComponent.SetMaterial` _staticmeshcomponent 0 "/Game/StarterContent/Materials/M_Metal_Steel.M_Metal_Steel")
    (`PrimitiveComponent.SetMaterial` _staticmeshcomponent 1 "/Game/StarterContent/Materials/M_Metal_Chrome.M_Metal_Chrome")
    (`PrimitiveComponent.SetMaterial` _staticmeshcomponent 2 "/Game/VRFireField/Material/Color_Red.Color_Red")
    (`PrimitiveComponent.SetMaterial` _staticmeshcomponent 3 "/Game/StarterContent/Materials/M_Metal_Steel.M_Metal_Steel")
    (`PrimitiveComponent.SetMaterial` _staticmeshcomponent 4 "/Game/StarterContent/Materials/M_Metal_Copper.M_Metal_Copper"))
  (`KismetSystemLibrary.Delay` 1.0)
  (goto _label_2))

(fn `UserConstructionScript`)