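; HarmfulSmoke is an escape-mode hazard volume that tells an Escape_Character when it enters or leaves smoke.
; Capsule overlap start calls InSmoke, while overlap end calls EndSmoke only if no other HarmfulSmoke still overlaps, so adjacent volumes chain cleanly.
; With FollowPlayer set, a fast looping timer runs CheckFollow, snapping the smoke onto an overlapping character while that character is inside a SmokeFollowVolume.
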(event `self.Capsule.OnComponentBeginOverlap`
  (params (OverlappedComponent :type "PrimitiveComponent Object Reference") (OtherActor :type "Actor Object Reference") (OtherComp :type "PrimitiveComponent Object Reference") (OtherBodyIndex :type Integer) (bFromSweep :type Boolean) (SweepResult :type "HitResult Structure (by ref)"))
  (bind _asescape_character (cast `/Game/VRFireField/Blueprint/EscapeMode/Escape_Character` OtherActor))
  (`/Game/VRFireField/Blueprint/EscapeMode/Escape_Character.InSmoke` _asescape_character))

(event `self.Capsule.OnComponentEndOverlap`
  (params (OverlappedComponent :type "PrimitiveComponent Object Reference") (OtherActor :type "Actor Object Reference") (OtherComp :type "PrimitiveComponent Object Reference") (OtherBodyIndex :type Integer))
  (bind _array_element (`/Game/MacroLibrary.ForEachLoopWithBreakOutput` (`self.GetOverlappingActors` OtherActor "HarmfulSmoke_C") :!label _label)
    (:`LoopBody`
      (cast `/Game/VRFireField/Blueprint/EscapeMode/HarmfulSmoke` _array_element)
      (goto _label :!via `Break`))
    (:`Completed`
      (bind _asescape_character (cast `/Game/VRFireField/Blueprint/EscapeMode/Escape_Character` OtherActor))
      (`/Game/VRFireField/Blueprint/EscapeMode/Escape_Character.EndSmoke` _asescape_character))))

(event `self.ReceiveBeginPlay`
  (if (`self.FollowPlayer`)
    (`KismetSystemLibrary.K2_SetTimer` null "CheckFollow" 0.02 true)))

(fn `CheckFollow`
  (bind _array_element (`/Game/MacroLibrary.ForEachLoopWithBreakOutput` (`PrimitiveComponent.GetOverlappingActors` (`self.Capsule`) null) :!label _label)
    (:`LoopBody`
      (bind _asescape_character (cast `/Game/VRFireField/Blueprint/EscapeMode/Escape_Character` _array_element))
      (goto _label :!via `Break`))
    (:`Breaked`
      (if (!= (`KismetArrayLibrary.Array_Length` (`self.GetOverlappingActors` _asescape_character "/Game/VRFireField/Blueprint/EscapeMode/SmokeFollowVolume.SmokeFollowVolume_C")) 0)
        (`self.K2_SetActorLocation` (`self.K2_GetActorLocation` _asescape_character))))))

(fn `UserConstructionScript`)