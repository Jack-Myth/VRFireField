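; WaterAmmo is a water projectile for the VR fire-field Escape Mode that delivers a "watered" message to what it strikes, then destroys itself.
; When MustHitPoint is set, it deactivates projectile movement and a timeline lerps it to HitLocation.
; Hits notify non-WaterBucket actors, or buckets when its own hit component is a sphere.
; Overlaps notify only through other actors' sphere components, with DoOnce gates limiting repeats.
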(event `self.ReceiveBeginPlay`
  (if (`self.MustHitPoint`)
    (`ActorComponent.Deactivate` (`self.ProjectileMovement`))
    (bind _output_get (set `self.InitalLocation` (`self.K2_GetActorLocation`)))
    (bind (_direction _lerpalpha) (`Timeline|ToHit` :!via `PlayFromStart`)
      (:`Update`
        (`self.K2_SetActorLocation` (`KismetMathLibrary.VLerp` _output_get (`self.HitLocation`) _lerpalpha))))))

(event `self.ReceiveHit`
  (params (MyComp :type "PrimitiveComponent Object Reference") (Other :type "Actor Object Reference") (OtherComp :type "PrimitiveComponent Object Reference") (bSelfMoved :type Boolean) (HitLocation :type "Vector Structure") (HitNormal :type "Vector Structure") (NormalImpulse :type "Vector Structure") (Hit :type "HitResult Structure (by ref)"))
  (bind _returnvalue (`GameplayStatics.GetObjectClass` Other))
  (`/Engine/EditorBlueprintResources/StandardMacros.DoOnce` false
    (:`Completed`
      (if (and (== (`GameplayStatics.GetObjectClass` MyComp) "/Script/Engine.SphereComponent") (== _returnvalue "/Game/VRFireField/Blueprint/EscapeMode/WaterBucket.WaterBucket_C"))
        (message `/Game/VRFireField/Blueprint/BaseObject/WaterableInterface.EventWeatered` Other)
        (`self.K2_DestroyActor` :!label _label)
        (elif (!= _returnvalue "/Game/VRFireField/Blueprint/EscapeMode/WaterBucket.WaterBucket_C")
          (message `/Game/VRFireField/Blueprint/BaseObject/WaterableInterface.EventWeatered` Other)
          (goto _label))))))

(event `self.StaticMeshComponent.OnComponentBeginOverlap`
  (params (OverlappedComponent :type "PrimitiveComponent Object Reference") (OtherActor :type "Actor Object Reference") (OtherComp :type "PrimitiveComponent Object Reference") (OtherBodyIndex :type Integer) (bFromSweep :type Boolean) (SweepResult :type "HitResult Structure (by ref)"))
  (`/Engine/EditorBlueprintResources/StandardMacros.DoOnce` false :!label _label_2
    (:`Completed`
      (if (== (`GameplayStatics.GetObjectClass` OtherComp) "/Script/Engine.SphereComponent")
        (message `/Game/VRFireField/Blueprint/BaseObject/WaterableInterface.EventWeatered` OtherActor)
        (`self.K2_DestroyActor`)
        (else
          (goto _label_2 :!via `Reset`))))))

(fn `UserConstructionScript`)