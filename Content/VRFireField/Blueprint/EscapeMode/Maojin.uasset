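; Maojin is a grabbable towel for the VR fire escape mode that can be wetted.
; Watering sets the wet flag, relabels it as a wet towel, records that in the GameInstance and alters the dynamic material's ColorMask.
; Grabbing swaps the mesh and opens the hand, also recording state if still dry; release restores the mesh.
; When wet, overlapping the escape character's Sphere10 component class calls InSMJ on that character.
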(event `/Game/VRFireField/Blueprint/BaseObject/WaterableInterface.EventWeatered`
  (set `self.Watered` true)
  (set `self.DisplayLable` "湿毛巾")
  (`/Game/VRFireField/Blueprint/TextR.SetText` (cast `/Game/VRFireField/Blueprint/TextR` (`WidgetComponent.GetUserWidgetObject` (`self.Widget`)) :!pure true) (`self.DisplayLable`))
  (set `/Game/VRFireField/Blueprint/DefaultGameInstance.湿毛巾` "NewEnumerator0" (`/Game/VRFireField/GameMacro.GetGameInstance`))
  (`MaterialInstanceDynamic.SetScalarParameterValue` (`self.MID`) "ColorMask" 0.3))

(event `self.Sphere.OnComponentBeginOverlap`
  (params (OverlappedComponent :type "PrimitiveComponent Object Reference") (OtherActor :type "Actor Object Reference") (OtherComp :type "PrimitiveComponent Object Reference") (OtherBodyIndex :type Integer) (bFromSweep :type Boolean) (SweepResult :type "HitResult Structure (by ref)"))
  (bind _asescape_character (cast `/Game/VRFireField/Blueprint/EscapeMode/Escape_Character` OtherActor))
  (if (and (== (`GameplayStatics.GetObjectClass` (`/Game/VRFireField/Blueprint/EscapeMode/Escape_Character.Sphere1_0` _asescape_character)) (`GameplayStatics.GetObjectClass` OtherComp)) (`self.Watered`))
    (`/Game/VRFireField/Blueprint/EscapeMode/Escape_Character.InSMJ` _asescape_character)))

(event `self.ReceiveBeginPlay`
  (`parent.ReceiveBeginPlay`)
  (bind _returnvalue (`PrimitiveComponent.CreateDynamicMaterialInstance` (`self.StaticMeshComponent`) 0 null))
  (set `self.MID` _returnvalue))

(event `self.BeginCatch`
  (params (HoldingHand :type "PrimitiveComponent Object Reference"))
  (bind _staticmeshcomponent (`self.StaticMeshComponent`))
  (`parent.BeginCatch` HoldingHand)
  (`StaticMeshComponent.SetStaticMesh` _staticmeshcomponent "/Game/VRFireField/Mesh/毛巾改.毛巾改")
  (`PrimitiveComponent.SetMaterial` _staticmeshcomponent 0 (`self.MID`))
  (bind _modelref (`/Game/VRFireField/Blueprint/FireFighter.GetHandModel` (`/Game/VRFireField/GameMacro.GetFireFighter`) HoldingHand))
  (`SkeletalMeshComponent.PlayAnimation` _modelref "/Game/VirtualReality/Mannequin/Animations/MannequinHand_Right_Open.MannequinHand_Right_Open" false)
  (if (not (`self.Watered`))
    (set `/Game/VRFireField/Blueprint/DefaultGameInstance.湿毛巾` "NewEnumerator1" (`/Game/VRFireField/GameMacro.GetGameInstance`))))

(event `self.EndCatch`
  (params (LastHoldHand :type "PrimitiveComponent Object Reference"))
  (bind _staticmeshcomponent (`self.StaticMeshComponent`))
  (`parent.EndCatch` LastHoldHand)
  (`StaticMeshComponent.SetStaticMesh` _staticmeshcomponent "/Game/VRFireField/Mesh/MAOJIN.MAOJIN")
  (`PrimitiveComponent.SetMaterial` _staticmeshcomponent 0 (`self.MID`)))

(fn `UserConstructionScript`
  (`parent.UserConstructionScript`))