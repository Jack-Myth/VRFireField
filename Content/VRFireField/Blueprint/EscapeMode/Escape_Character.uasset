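; VR player character for a fire-escape mode, handling fire and smoke hazards and arrival at the exit.
; Fire or smoke starts a warning, sound and gradual camera fade that reverses on escape, or ends in death, a counted attempt and level reload.
; A wet towel, polled via Sphere10 overlap, blocks smoke.
; Tick moves the actor by headset XY delta with counter-offset VROffset; exit triggers LevelResult checks or a pass message.
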(event `StartDie`
  (params (FadeColor :type "LinearColor Structure") (DiedMessage :type String))
  (bind _returnvalue (`GameplayStatics.GetPlayerCameraManager` 0))
  (bind _fadeprocess (`self.FadeProcess`))
  (bind _fadetime (`self.FadeTime`))
  ;[1 1 1] Die
  (`/Engine/EditorBlueprintResources/StandardMacros.DoOnce` false :!label _label
    (:`Completed`
      (`|ExecutionSequence`
        (:`then_0`
          (goto _label_3 :!via `Break`))
        (:`then_1`
          (bind _widgethandle (`/Game/VRFireField/GameMacro.ShowMessage` "快远离火焰" -1.0)
            (:`Out`
              (bind _returnvalue_2 (`GameplayStatics.SpawnSound2D` "/Game/VRFireField/Sound/Hitted.Hitted"))
              (`AudioComponent.Play` _returnvalue_2 0.0))))
        (:`then_2`
          (bind _index (`/Game/MacroLibrary.ForLoopWithDelay` _fadeprocess 50 (/ _fadetime 50.0) :!label _label_2)
            (:`LoopBody`
              (set `self.FadeProcess` _index)
              (`PlayerCameraManager.SetManualCameraFade` _returnvalue (* _index 0.02) FadeColor false))
            (:`Complited`
              (set `self.Dying` true)
              (`KismetSystemLibrary.Delay` 1.0)
              (bind _returnvalue_3 (`|CreateWidget` "/Game/VRFireField/Blueprint/BaseObject/Text2DViewport.Text2DViewport_C"))
              (`/Game/VRFireField/Blueprint/BaseObject/Text2DViewport.SetText` _returnvalue_3 DiedMessage)
              (`WidgetLayoutLibrary.RemoveAllWidgets`)
              (`UserWidget.AddToViewport` _returnvalue_3 0)
              (`self.DisableInput` (`GameplayStatics.GetPlayerController` 0))
              (`KismetSystemLibrary.Delay` 2.0)
              (`/Engine/EditorBlueprintResources/StandardMacros.IncrementInt` (`/Game/VRFireField/Blueprint/DefaultGameInstance.EscapeCount` (`/Game/VRFireField/GameMacro.GetGameInstance`))
                (:`  `
                  (bind _returnvalue_4 (`GameplayStatics.GetCurrentLevelName` true))
                  (`GameplayStatics.OpenLevel` (`KismetStringLibrary.Conv_StringToName` _returnvalue_4)))))))))))

(event `Key|LeftControl`
  (params (Key :type "Key Structure" :default "AnyKey")))

(event `StopDie`
  ;[1 1 1] Die
  (if (not (`self.Dying`))
    (`|ExecutionSequence`
      (:`then_0`
        (goto _label_2 :!via `Break`))
      (:`then_1`
        (`Widget.RemoveFromParent` (stale `StartDie` _widgethandle))
        (`AudioComponent.Stop` (stale `StartDie` _returnvalue_2))
        (goto _label :!via `Reset`))
      (:`then_2`
        (bind _index (`/Game/MacroLibrary.ForLoopWithDelay` (- 50 (`self.FadeProcess`)) 50 (/ (`self.FadeTime`) 50.0) :!label _label_3)
          (:`LoopBody`
            (bind _returnvalue (- 50 _index))
            (set `self.FadeProcess` _returnvalue)
            (`PlayerCameraManager.SetManualCameraFade` (`GameplayStatics.GetPlayerCameraManager` 0) (* _returnvalue 0.02) (stale `StartDie` FadeColor) false)))))))

(event `self.ReceiveTick`
  (params (DeltaSeconds :type "Float (single-precision)"))
  (bind (_devicerotation _deviceposition) (`HeadMountedDisplayFunctionLibrary.GetOrientationAndPosition`))
  (bind (_returnvalue_x _returnvalue_y _returnvalue_z) (`KismetMathLibrary.BreakVector` (`self.K2_GetActorLocation`)))
  (bind (_devicerotation_2 _deviceposition_2) (`HeadMountedDisplayFunctionLibrary.GetOrientationAndPosition`))
  (bind _vroffset (`self.VROffset`))
  (bind (_returnvalue_x_2 _returnvalue_y_2) (`KismetMathLibrary.BreakVector` (- _deviceposition_2 (`self.PersonLastPosition`))))
  (bind (_relativelocation_x _relativelocation_y _relativelocation_z) (`KismetMathLibrary.BreakVector` (`SceneComponent.RelativeLocation` _vroffset)))
  ;[1 1 1] Tick
  (if (`HeadMountedDisplayFunctionLibrary.IsHeadMountedDisplayEnabled`)
    (`self.K2_SetActorLocation` (`KismetMathLibrary.MakeVector` (+ _returnvalue_x _returnvalue_x_2) (+ _returnvalue_y _returnvalue_y_2) _returnvalue_z) true)
    (`SceneComponent.K2_SetRelativeLocation` _vroffset (`KismetMathLibrary.MakeVector` (* -1 (.x _deviceposition)) (* -1 (.y _deviceposition)) _relativelocation_z) false false)
    (set `self.PersonLastPosition` _deviceposition_2)))

(event `InSMJ`
  (set `self.SMaojin` true)
  (`self.EndSmoke`)
  (`KismetSystemLibrary.K2_SetTimer` null "CheckSMJ" 0.02 true)
  (`/Engine/EditorBlueprintResources/StandardMacros.DoOnce` false
    (:`Completed`
      (set `/Game/VRFireField/Blueprint/DefaultGameInstance.捂嘴` "NewEnumerator0" (`/Game/VRFireField/GameMacro.GetGameInstance`)))))

(event `ArriveExit`
  ;[1 1 1] ArriveExit
  (`/Engine/EditorBlueprintResources/StandardMacros.DoOnce` false
    (:`Completed`
      (set `CharacterMovementComponent.MaxWalkSpeed` 0.1 (`self.CharacterMovement`))
      (bind _outactors (`GameplayStatics.GetAllActorsOfClass` "/Game/VRFireField/Blueprint/SenceObject/LevelResult.LevelResult_C"))
      (`/Game/VRFireField/Blueprint/SenceObject/LevelResult.BeginCheckResult` _outactors)
      (if (< (`KismetArrayLibrary.Array_Length` _outactors) 1)
        (`PlayerCameraManager.StartCameraFade` (`GameplayStatics.GetPlayerCameraManager` 0) 0.0 0.7 1.0 (struct :`G` 0.024377 :`B` 0.3 :`A` 1.0) false true)
        (bind _returnvalue (`|CreateWidget` "/Game/VRFireField/Blueprint/BaseObject/Text2DViewport.Text2DViewport_C"))
        (`/Game/VRFireField/Blueprint/BaseObject/Text2DViewport.SetText` _returnvalue "过关！")
        (`UserWidget.AddToViewport` _returnvalue 0)))))

(event `InSmoke`
  (bind _returnvalue (`GameplayStatics.GetPlayerCameraManager` 0))
  (bind _fadeprocess (`self.FadeProcess`))
  (bind _fadesmoketime (`self.FadeSmokeTime`))
  (`/Engine/EditorBlueprintResources/StandardMacros.DoOnce` false :!label _label_4
    (:`Completed`
      (if (not (`self.SMaojin`))
        (bind _widgethandle (`/Game/VRFireField/GameMacro.ShowMessage` "快用湿毛巾捂住口鼻" -1.0)
          (:`Out`
            (bind _returnvalue_2 (`GameplayStatics.SpawnSound2D` "/Game/VRFireField/Sound/咳嗽.咳嗽"))
            (`AudioComponent.Play` _returnvalue_2 0.0)
            (`|ExecutionSequence`
              (:`then_0`
                (set `/Game/VRFireField/Blueprint/DefaultGameInstance.捂嘴` "NewEnumerator1" (`/Game/VRFireField/GameMacro.GetGameInstance`)))
              (:`then_1`
                (goto _label_6 :!via `Break`))
              (:`then_2`
                (bind _index (`/Game/MacroLibrary.ForLoopWithDelay` _fadeprocess 50 (/ _fadesmoketime 50.0) :!label _label_5)
                  (:`LoopBody`
                    (set `self.FadeProcess` _index)
                    (`PlayerCameraManager.SetManualCameraFade` _returnvalue (* _index 0.02) (struct :`A` 1.0) false))
                  (:`Complited`
                    (set `self.Dying` true)
                    (`KismetSystemLibrary.Delay` 1.0)
                    (bind _returnvalue_3 (`|CreateWidget` "/Game/VRFireField/Blueprint/BaseObject/Text2DViewport.Text2DViewport_C"))
                    (`/Game/VRFireField/Blueprint/BaseObject/Text2DViewport.SetText` _returnvalue_3 "遇到烟雾需用湿毛巾捂住口鼻")
                    (`WidgetLayoutLibrary.RemoveAllWidgets`)
                    (`UserWidget.AddToViewport` _returnvalue_3 0)
                    (`self.DisableInput` (`GameplayStatics.GetPlayerController` 0))
                    (`/Engine/EditorBlueprintResources/StandardMacros.IncrementInt` (`/Game/VRFireField/Blueprint/DefaultGameInstance.EscapeCount` (`/Game/VRFireField/GameMacro.GetGameInstance`))
                      (:`  `
                        (`KismetSystemLibrary.Delay` 2.0)
                        (bind _returnvalue_4 (`GameplayStatics.GetCurrentLevelName` true))
                        (`GameplayStatics.OpenLevel` (`KismetStringLibrary.Conv_StringToName` _returnvalue_4))))))))))))))

(event `EndSmoke`
  (`|ExecutionSequence`
    (:`then_0`
      (goto _label_4 :!via `Reset`))
    (:`then_1`
      (`/Engine/EditorBlueprintResources/StandardMacros.IsValid` (stale `InSmoke` _widgethandle)
        (:`Is Valid`
          (`Widget.RemoveFromParent` (stale `InSmoke` _widgethandle))
          (`AudioComponent.Stop` (stale `InSmoke` _returnvalue_2)))
        (:`Is Not Valid`
          _))
      (if (not (`self.Dying`))
        (`|ExecutionSequence`
          (:`then_0`
            (goto _label_5 :!via `Break`))
          (:`then_1`
            (bind _index (`/Game/MacroLibrary.ForLoopWithDelay` (- 50 (`self.FadeProcess`)) 50 (/ (`self.FadeSmokeTime`) 50.0) :!label _label_6)
              (:`LoopBody`
                (bind _returnvalue (- 50 _index))
                (set `self.FadeProcess` _returnvalue)
                (`PlayerCameraManager.SetManualCameraFade` :`self` (`GameplayStatics.GetPlayerCameraManager` 0) :`InFadeAmount` (* _returnvalue 0.02))))))))))

(fn `CheckSMJ`
  (if (not (> (`KismetArrayLibrary.Array_Length` (`PrimitiveComponent.GetOverlappingActors` (`self.Sphere1_0`) "/Game/VRFireField/Blueprint/EscapeMode/Maojin.Maojin_C")) 0))
    (set `self.SMaojin` false)
    (`KismetSystemLibrary.K2_ClearTimer` null "CheckSMJ")))

(fn `UserConstructionScript`
  (`parent.UserConstructionScript`))