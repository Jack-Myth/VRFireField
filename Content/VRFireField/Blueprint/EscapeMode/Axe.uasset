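; A grabbable fire axe for the VR fire escape mode that damages breakable boxes.
; When its capsule overlaps a BreakableBox while the mesh is attached to a parent, it applies fixed damage, crediting the owner of that parent as the causer.
; On grab, it runs the parent catch logic and then sets the fire axe (消防斧) enum state on the GameInstance.
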(event `self.Capsule.OnComponentBeginOverlap`
  (params (OverlappedComponent :type "PrimitiveComponent Object Reference") (OtherActor :type "Actor Object Reference") (OtherComp :type "PrimitiveComponent Object Reference") (OtherBodyIndex :type Integer) (bFromSweep :type Boolean) (SweepResult :type "HitResult Structure (by ref)"))
  (bind _returnvalue (`SceneComponent.GetAttachParent` (`self.StaticMeshComponent`)))
  (bind _asbreakable_box (cast `/Game/VRFireField/Blueprint/EscapeMode/BreakableBox` OtherActor))
  (`/Engine/EditorBlueprintResources/StandardMacros.IsValid` _returnvalue
    (:`Is Valid`
      (`GameplayStatics.ApplyDamage` _asbreakable_box 50.0 null (`ActorComponent.GetOwner` _returnvalue)))))

(event `self.BeginCatch`
  (params (HoldingHand :type "PrimitiveComponent Object Reference"))
  (`parent.BeginCatch` null)
  (set `/Game/VRFireField/Blueprint/DefaultGameInstance.消防斧` "NewEnumerator0" (`/Game/VRFireField/GameMacro.GetGameInstance`)))

(fn `UserConstructionScript`
  (`parent.UserConstructionScript`))