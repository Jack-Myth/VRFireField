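; VR water bucket for the fire field's escape mode that throws its water when swung while in use.
; A watering event shows the water sphere, which doubles as the filled state.
; A fast looping timer derives velocity from position changes and fires when motion toward a Scene component passes a threshold.
; It spawns WaterAmmo with swing-based velocity, or passes it a forced hit point, then hides the sphere.
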(event `/Game/VRFireField/Blueprint/BaseObject/WaterableInterface.EventWeatered`
  (`SceneComponent.SetHiddenInGame` (`self.Sphere`) false false))

(event `self.ReceiveBeginPlay`
  (`parent.ReceiveBeginPlay`)
  (set `self.LastPosition` (`self.K2_GetActorLocation`))
  (`KismetSystemLibrary.K2_SetTimerDelegate` (delegate `CheckShootWater`) 0.02 true))

(event `self.BeginUse`
  (params (HoldingHand :type "PrimitiveComponent Object Reference"))
  (set `self.Throwable` true))

(event `self.EndUse`
  (params (HouldingHand :type "PrimitiveComponent Object Reference"))
  (set `self.Throwable` false))

(event `CheckShootWater`
  (bind _returnvalue (`self.K2_GetActorLocation`))
  (bind _musthitpoint (`self.MustHitPoint`))
  (bind _returnvalue_2 (- (`SceneComponent.K2_GetComponentLocation` (`self.Scene`)) (`self.K2_GetActorLocation`)))
  (bind _output_get (set `self.Speed_0` (* (- _returnvalue (`self.LastPosition`)) 50)))
  (set `self.LastPosition` _returnvalue)
  (if (and (and (> (`KismetMathLibrary.Dot_VectorVector` _output_get _returnvalue_2) 200.0) (not (`SceneComponent.bHiddenInGame` (`self.Sphere`)))) (`self.Throwable`))
    ;[1 1 1] Shoot
    (bind _returnvalue_3 (`|SpawnActorFromClass` "/Game/VRFireField/Blueprint/EscapeMode/WaterAmmo.WaterAmmo_C" (`KismetMathLibrary.MakeTransform` (`SceneComponent.K2_GetComponentLocation` (`self.Scene1`)) (struct) (1.0 1.0 1.0)) "AlwaysSpawn" "OverrideRootScale" null _musthitpoint (`self.HitLocation`)))
    (if (not _musthitpoint)
      (bind _projectilemovement (`/Game/VRFireField/Blueprint/EscapeMode/WaterAmmo.ProjectileMovement` _returnvalue_3))
      (set `MovementComponent.Velocity` (+ (* _output_get 1.8) (* _returnvalue_2 (/ (`KismetMathLibrary.VSize` _output_get) 50.0))) _projectilemovement)
      (`ActorComponent.SetActive` _projectilemovement true false))
    (`SceneComponent.SetHiddenInGame` (`self.Sphere`) true false)))

(fn `UserConstructionScript`
  (`parent.UserConstructionScript`))