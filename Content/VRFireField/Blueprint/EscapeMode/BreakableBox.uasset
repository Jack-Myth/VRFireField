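; Breakable box in escape mode that only takes damage from a FireFighter, playing a chop sound per hit until its health runs out.
; On breaking, it hides itself and spawns a destructible actor with its fracture mesh, shattered along the right motion controller's forward vector with damage and impulse scaled by average box scale.
; The debris ignores pawns, and after a delay the box calls OnBreaked and destroys both actors.
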(event `self.ReceiveAnyDamage`
  (params (Damage :type "Float (single-precision)") (DamageType :type "DamageType Object Reference") (InstigatedBy :type "Controller Object Reference") (DamageCauser :type "Actor Object Reference"))
  (bind _returnvalue (`self.K2_GetActorLocation`))
  (bind (_returnvalue_x _returnvalue_y _returnvalue_z) (`KismetMathLibrary.BreakVector` (`self.GetActorScale3D`)))
  (bind _returnvalue_2 (* 1000 (/ (+ (+ _returnvalue_x _returnvalue_y) _returnvalue_z) 3.0)))
  (bind _asfire_fighter (cast `/Game/VRFireField/Blueprint/FireFighter` DamageCauser))
  (bind _output_get (set `self.Health` (- (`self.Health`) Damage)))
  (if (<= _output_get 0.0)
    (`GameplayStatics.PlaySoundAtLocation` "/Game/VRFireField/Sound/金属重砍木头.金属重砍木头" _returnvalue (struct) 1.0 1.0 0.0 "/Game/VRFireField/Blueprint/DefaultSoundAttenuation.DefaultSoundAttenuation")
    (`self.SetActorEnableCollision` false)
    (`self.SetActorHiddenInGame` true)
    (`PrimitiveComponent.SetSimulatePhysics` (`self.StaticMeshComponent`) false)
    (bind _returnvalue_3 (`|SpawnActorFromClass` "/Script/Engine.DestructibleActor" (`self.GetTransform`) "Undefined" "OverrideRootScale"))
    (bind _destructiblecomponent (`DestructibleActor.DestructibleComponent` _returnvalue_3))
    (`DestructibleComponent.SetDestructibleMesh` _destructiblecomponent (`self.DestributeMesh`))
    (`DestructibleComponent.ApplyDamage` _destructiblecomponent _returnvalue_2 (`self.K2_GetActorLocation` _returnvalue_3) (`SceneComponent.GetForwardVector` (`/Game/VRFireField/Blueprint/FireFighter.MotionController_R` _asfire_fighter)) _returnvalue_2)
    (`PrimitiveComponent.SetCollisionResponseToChannel` _destructiblecomponent "ECC_Pawn" "ECR_Ignore")
    (`KismetSystemLibrary.Delay` 5.0)
    (`self.OnBreaked` self)
    (`self.K2_DestroyActor` _returnvalue_3)
    (`self.K2_DestroyActor` self)
    (else
      (`GameplayStatics.PlaySoundAtLocation` "/Game/VRFireField/Sound/金属砍木头.金属砍木头" _returnvalue (struct) 1.0 1.0 0.0 "/Game/VRFireField/Blueprint/DefaultSoundAttenuation.DefaultSoundAttenuation"))))

(fn `UserConstructionScript`)