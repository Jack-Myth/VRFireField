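; World-space progress bar actor for Escape Mode that wraps a FloatingProgressBarWidget in a widget component.
; It forwards set, increment, decrement and color calls to the widget, clamping set values to 0–1.
; On BeginPlay it binds the widget's max and empty events and re-broadcasts them as its own.
; When FollowPlayer is set, it enables Tick to yaw toward the player pawn.
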(event `self.ReceiveBeginPlay`
  (bind _asfloating_progress_bar_widget (cast `/Game/VRFireField/Blueprint/EscapeMode/FloatingProgressBarWidget` (`WidgetComponent.GetUserWidgetObject` (`self.Widget`)) :!pure true))
  (add `/Game/VRFireField/Blueprint/EscapeMode/FloatingProgressBarWidget.EventMax` _asfloating_progress_bar_widget (delegate `EventMax_0`))
  (add `/Game/VRFireField/Blueprint/EscapeMode/FloatingProgressBarWidget.EventEmpty` _asfloating_progress_bar_widget (delegate `EventEmpty_0`))
  (if (`self.FollowPlayer`)
    (`self.SetActorTickEnabled` true)))

(event `SetProgressValue`
  (params (`New Value` :type "Float (double-precision)"))
  (bind _asfloating_progress_bar_widget (cast `/Game/VRFireField/Blueprint/EscapeMode/FloatingProgressBarWidget` (`WidgetComponent.GetUserWidgetObject` (`self.Widget`))))
  (`/Game/VRFireField/Blueprint/EscapeMode/FloatingProgressBarWidget.SetProgressValue` _asfloating_progress_bar_widget (`KismetMathLibrary.FClamp` `New Value`)))

(event `EventMax_0`
  (`self.EventMax`))

(event `EventEmpty_0`
  (`self.EventEmpty`))

(event `Increment`
  (params (Value :type "Float (double-precision)"))
  (bind _asfloating_progress_bar_widget (cast `/Game/VRFireField/Blueprint/EscapeMode/FloatingProgressBarWidget` (`WidgetComponent.GetUserWidgetObject` (`self.Widget`))))
  (`/Game/VRFireField/Blueprint/EscapeMode/FloatingProgressBarWidget.Increment` _asfloating_progress_bar_widget Value))

(event `Decrement`
  (params (Value :type "Float (double-precision)"))
  (bind _asfloating_progress_bar_widget (cast `/Game/VRFireField/Blueprint/EscapeMode/FloatingProgressBarWidget` (`WidgetComponent.GetUserWidgetObject` (`self.Widget`))))
  (`/Game/VRFireField/Blueprint/EscapeMode/FloatingProgressBarWidget.Decrement` _asfloating_progress_bar_widget Value))

(event `self.ReceiveTick`
  (params (DeltaSeconds :type "Float (single-precision)"))
  (bind (_returnvalue_roll _returnvalue_pitch _returnvalue_yaw) (`KismetMathLibrary.BreakRotator` (`KismetMathLibrary.FindLookAtRotation` (`self.K2_GetActorLocation`) (`self.K2_GetActorLocation` (`GameplayStatics.GetPlayerPawn` 0)))))
  (`self.K2_SetActorRotation` (`KismetMathLibrary.MakeRotator` 0.0 0.0 _returnvalue_yaw)))

(event `SetColor`
  (params (Fade :type Boolean) (`Static Color` :type "LinearColor Structure") (ColorMax :type "LinearColor Structure") (ColorMin :type "LinearColor Structure"))
  (bind _asfloating_progress_bar_widget (cast `/Game/VRFireField/Blueprint/EscapeMode/FloatingProgressBarWidget` (`WidgetComponent.GetUserWidgetObject` (`self.Widget`))))
  (`/Game/VRFireField/Blueprint/EscapeMode/FloatingProgressBarWidget.SetColor` _asfloating_progress_bar_widget Fade `Static Color` ColorMax ColorMin))

(fn `UserConstructionScript`)