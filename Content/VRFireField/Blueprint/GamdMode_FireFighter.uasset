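; Game mode for the VR firefighter game that enables the HMD on start, sets shadow, texture and streaming pool console settings, and manages dynamic render resolution.
; Tick derives FPS from frame time, and a looping timer compares it to low and high thresholds to step the Screen value down or up for an r.ScreenPercentage console command.
; The -WithoutDynamicRSP command line switch disables the timer.
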(event `self.ReceiveBeginPlay`
  (`HeadMountedDisplayFunctionLibrary.EnableHMD` true)
  (`KismetSystemLibrary.ExecuteConsoleCommand` "sg.ShadowQuality 1")
  (`KismetSystemLibrary.ExecuteConsoleCommand` "sg.TextureQuality 3")
  (`KismetSystemLibrary.ExecuteConsoleCommand` "r.Streaming.PoolSize 4000")
  (bind _returnvalue (`KismetSystemLibrary.GetCommandLine`))
  (if (not (`KismetStringLibrary.Contains` _returnvalue "-WithoutDynamicRSP"))
    (`KismetSystemLibrary.K2_SetTimerDelegate` (delegate `TickForDynamicRSP`) 0.2 true)))

(event `TickForDynamicRSP`
  (bind _fps (`self.FPS`))
  (bind _screen_ (`self.Screen%`))
  (if (< _fps 40)
    (if (> _screen_ 70)
      (bind _output_get (set `self.Screen%` (- _screen_ 15)))
      (`KismetSystemLibrary.ExecuteConsoleCommand` (`KismetStringLibrary.Concat_StrStr` "r.ScreenPercentage " (`KismetStringLibrary.Conv_IntToString` _output_get))))
    (elif (and (> _fps 55) (< _screen_ 100))
      (bind _output_get_2 (set `self.Screen%` (+ _screen_ 15)))
      (`KismetSystemLibrary.ExecuteConsoleCommand` (`KismetStringLibrary.Concat_StrStr` "r.ScreenPercentage " (`KismetStringLibrary.Conv_IntToString` _output_get_2))))))

(event `self.ReceiveTick`
  (params (DeltaSeconds :type "Float (single-precision)"))
  (set `self.FPS` (`KismetMathLibrary.FTrunc` (/ 1.0 DeltaSeconds))))

(fn `UserConstructionScript`)