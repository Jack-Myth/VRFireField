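; Pot lid (锅盖) actor that damages fires it overlaps and triggers their re-fire when removed.
; On begin overlap it applies a fixed amount of damage to any Fire_锅 (pot fire), or to a Fire actor listed in ExtraActorToDamage.
; On end overlap the same targets receive a ReFire call.
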(event `self.ReceiveActorBeginOverlap`
  (params (OtherActor :type "Actor Object Reference"))
  (bind `_asfire_锅` (cast `/Game/VRFireField/Blueprint/Fire_锅` OtherActor)
    (:`then`
      (`GameplayStatics.ApplyDamage` `_asfire_锅` 3.0))
    (:`CastFailed`
      (if (`KismetArrayLibrary.Array_Contains` (`self.ExtraActorToDamage`) OtherActor)
        (bind _asfire (cast `/Game/VRFireField/Blueprint/Fire` OtherActor))
        (`GameplayStatics.ApplyDamage` _asfire 3.0)))))

(event `self.ReceiveActorEndOverlap`
  (params (OtherActor :type "Actor Object Reference"))
  (bind `_asfire_锅` (cast `/Game/VRFireField/Blueprint/Fire_锅` OtherActor)
    (:`then`
      (`/Game/VRFireField/Blueprint/Fire_锅.ReFire` `_asfire_锅`))
    (:`CastFailed`
      (if (`KismetArrayLibrary.Array_Contains` (`self.ExtraActorToDamage`) OtherActor)
        (bind _asfire (cast `/Game/VRFireField/Blueprint/Fire` OtherActor))
        (`/Game/VRFireField/Blueprint/Fire_锅.ReFire` _asfire)))))

(fn `UserConstructionScript`)