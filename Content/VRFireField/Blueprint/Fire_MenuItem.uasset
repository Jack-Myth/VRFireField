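; Level-select menu item for the VR fire game that loads a level through a spawned Fire actor.
; On BeginPlay it spawns a Fire at its own transform and a half-scale, non-following FloatingText label above it showing the item's Text.
; It binds to the Fire's OnReadyToDistory dispatcher, and when that fires it waits briefly and opens LevelToLoad by name.
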(event `self.ReceiveBeginPlay`
  (bind _returnvalue (`self.K2_GetActorLocation`))
  (bind _returnvalue_2 (`self.K2_GetActorRotation`))
  (bind _returnvalue_3 (`|SpawnActorFromClass` "/Game/VRFireField/Blueprint/Fire.Fire_C" (`KismetMathLibrary.MakeTransform` _returnvalue _returnvalue_2) "Undefined" "OverrideRootScale" null 1.0))
  (bind _output_get (set `self.FireRef` _returnvalue_3))
  (add `/Game/VRFireField/Blueprint/Fire.OnReadyToDistory` _output_get (delegate `ReadyToLoad`))
  (`|SpawnActorFromClass` "/Game/VRFireField/Blueprint/SenceObject/FloatingText.FloatingText_C" (`KismetMathLibrary.MakeTransform` (+ _returnvalue (0.0 0.0 72.0)) _returnvalue_2 (0.5 0.5 0.5)) "Undefined" "OverrideRootScale" null (`self.Text`)))

(event `ReadyToLoad`
  (`KismetSystemLibrary.Delay` 1.0)
  (`GameplayStatics.OpenLevel` (`self.LevelToLoad`)))

(fn `UserConstructionScript`)